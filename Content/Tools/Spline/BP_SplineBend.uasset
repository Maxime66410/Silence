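; BP_SplineBend is a spline tool that bends a static mesh along a spline in repeated sections.
; Its construction script adds one spline mesh per SectionLength, applying the configured mesh, material, forward axis and collision setting.
; Segment ends sample location and length-clamped tangents by distance, while scale reads the spline point matching the segment index.
; ExportStaticMesh is an empty function.
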(fn `ExportStaticMesh`)

(fn `UserConstructionScript`
  (bind _sectionlength (`self.SectionLength`))
  (bind _spline (`self.Spline`))
  (bind _coordinatespace (`self.CoordinateSpace`))
  (for _index (range (`KismetMathLibrary.Round` (/ (`SplineComponent.GetSplineLength` (`self.Spline`)) (`self.SectionLength`))))
    (bind _returnvalue (`AddComponent|NODE_AddSplineMeshComponent-0`))
    (`StaticMeshComponent.SetStaticMesh` _returnvalue (`self.StaticMesh`))
    (`PrimitiveComponent.SetMaterial` _returnvalue 0 (`self.Material`))
    (`SplineMeshComponent.SetForwardAxis` _returnvalue (`self.ForwardAxis`) true)
    (bind _returnvalue_2 (`KismetMathLibrary.Conv_VectorToVector2D` (* (`SplineComponent.GetScaleAtSplinePoint` (`self.Spline`) _index) (`self.Scale`))))
    (`SplineMeshComponent.SetStartScale` _returnvalue _returnvalue_2 true)
    (`SplineMeshComponent.SetEndScale` _returnvalue _returnvalue_2 true)
    (bind _returnvalue_3 (* _index _sectionlength))
    (bind _returnvalue_4 (* (+ _index 1) _sectionlength))
    (`SplineMeshComponent.SetStartAndEnd` _returnvalue (`SplineComponent.GetLocationAtDistanceAlongSpline` _spline _returnvalue_3 _coordinatespace) (`KismetMathLibrary.ClampVectorSize` (`SplineComponent.GetTangentAtDistanceAlongSpline` _spline _returnvalue_3 _coordinatespace) 0.0 (`self.SectionLength`)) (`SplineComponent.GetLocationAtDistanceAlongSpline` _spline _returnvalue_4 _coordinatespace) (`KismetMathLibrary.ClampVectorSize` (`SplineComponent.GetTangentAtDistanceAlongSpline` _spline _returnvalue_4 _coordinatespace) 0.0 (`self.SectionLength`)) true)
    (`PrimitiveComponent.SetCollisionEnabled` _returnvalue (`self.CollisionEnabled`))))