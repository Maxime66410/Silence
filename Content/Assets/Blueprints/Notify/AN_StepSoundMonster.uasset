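; Animation notify that plays a monster's footstep sound at the ground beneath it.
; It runs a complex Visibility line trace from the owner's location down along its up axis, ignoring the owner.
; On a hit, it plays a quiet concrete walk sound at the impact location with attenuation.
; The same sound plays regardless of the surface hit.
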(fn `Received_Notify`
  (params (MeshComp :type "SkeletalMeshComponent Object Reference") (Animation :type "AnimSequenceBase Object Reference") (EventReference :type "AnimNotifyEventReference Structure (by ref)"))
  (returns (ReturnValue :type Boolean))
  (bind _returnvalue (`ActorComponent.GetOwner` MeshComp))
  (bind _returnvalue_2 (`Actor.K2_GetActorLocation` _returnvalue))
  (bind (_outhit _returnvalue_3) (`KismetSystemLibrary.LineTraceSingle` _returnvalue_2 (+ _returnvalue_2 (* (`Actor.GetActorUpVector` _returnvalue) -110.0)) "TraceTypeQuery1" true (`|MakeArray` _returnvalue)))
  (if _returnvalue_3
    (`GameplayStatics.PlaySoundAtLocation` "/Game/Assets/Audio/Player/Step/Walk/SC_footstep_concrete_walk.SC_footstep_concrete_walk" (`.Location` (`GameplayStatics.BreakHitResult` _outhit)) (struct) 0.25 1.0 0.0 "/Game/Assets/Audio/Attenuation/SA_High.SA_High" null null null)
    (return true)))