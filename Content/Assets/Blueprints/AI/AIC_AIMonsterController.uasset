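; AI controller for the monster that runs its behavior tree and hunts the first-person player by sound.
; Loud enough hearing stimuli write a sound location to the blackboard, and the loudest ones with the player nearby also enable chasing the player.
; The Screamer event stops movement, flags the player dead, attaches a spawned camera to the monster's skeleton for a jumpscare view, and plays a scream montage.
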(event `self.ReceiveBeginPlay`
  (`self.RunBehaviorTree` "/Game/Assets/Blueprints/AI/BT_AIMonster.BT_AIMonster")
  (`self.GetPlayer`))

(event `self.AIPerception.OnTargetPerceptionUpdated`
  (params (Actor :type "Actor Object Reference") (Stimulus :type "AIStimulus Structure"))
  (`self.HandleHearing` Actor Stimulus))

(event `StopFollowPlayer`
  (`BlackboardComponent.SetValueAsBool` (`self.Blackboard`) "ChasePlayer" false)
  (`BlackboardComponent.SetValueAsBool` (`self.Blackboard`) "CanAttack" false)
  (`BlackboardComponent.SetValueAsBool` (`self.Blackboard`) "LaunchGame" false))

(event `Screamer`
  (`self.StopMovement`)
  (bind _player (`self.Player`)
    (:`then`
      (if (not (`/Game/Assets/Blueprints/Player/BP_FirstPersonCharacter.IsDeath` _player))
        (set `/Game/Assets/Blueprints/Player/BP_FirstPersonCharacter.IsDeath` true _player)
        (`self.SyncCam`)
        (bind _asbp_aimonster (cast `/Game/Assets/Blueprints/AI/BP_AIMonster` (`self.K2_GetPawn`)))
        (`|PlayMontage` (`Character.Mesh` _asbp_aimonster) "/Game/Assets/Animations/ZombieFisherman_Torch_Scream_Montage.ZombieFisherman_Torch_Scream_Montage")))
    (:`else`)))

(fn `GetPlayer`
  (bind _returnvalue (`GameplayStatics.GetActorOfClass` "/Game/Assets/Blueprints/Player/BP_FirstPersonCharacter.BP_FirstPersonCharacter_C"))
  (set `self.Player` _returnvalue))

(fn `HandleHearing`
  (params (Actor :type "Actor Object Reference") (Stimulus :type "AIStimulus Structure"))
  (bind _blackboard (`self.Blackboard`))
  (bind _blackboard_2 (`self.Blackboard`))
  (bind (_age _expirationage _strength _stimuluslocation _receiverlocation) (break `AIStimulus` (`local.Stimulus`)))
  (bind _returnvalue (`AIPerceptionSystem.GetSenseClassForStimulus` Stimulus))
  (if (== _returnvalue "/Script/AIModule.AISense_Hearing")
    (if (>= _strength 0.6)
      (`BlackboardComponent.SetValueAsVector` _blackboard "SoundLocation" _stimuluslocation)
      (`BlackboardComponent.SetValueAsBool` _blackboard "ChaseSound" true)
      (bind _player (`self.Player`)
        (:`then`
          (if (and (<= (`KismetMathLibrary.Vector_Distance` _receiverlocation (`self.K2_GetActorLocation` _player)) 500.0) (>= _strength 1.0))
            (`BlackboardComponent.SetValueAsObject` _blackboard_2 "Player" _player)
            (`BlackboardComponent.SetValueAsBool` _blackboard_2 "ChasePlayer" true)
            (else
              (`BlackboardComponent.SetValueAsBool` _blackboard_2 "ChasePlayer" false))))
        (:`else`
          (`self.GetPlayer`))))))

(fn `SyncCam`
  (locals (LocalCamera :type "CameraActor Object Reference"))
  (bind _asbp_aimonster (cast `/Game/Assets/Blueprints/AI/BP_AIMonster` (`self.K2_GetPawn`)))
  (bind _returnvalue (`|SpawnActorFromClass` "/Script/Engine.CameraActor" (`KismetMathLibrary.MakeTransform` (0.0 0.0 0.0)) "AlwaysSpawn" "MultiplyWithRoot" null null))
  (bind _output_get (set `local.LocalCamera` _returnvalue))
  (`self.K2_AttachToComponent` _output_get (`Character.Mesh` _asbp_aimonster) "CATRigHub003" "SnapToTarget" "SnapToTarget" "SnapToTarget" true)
  (`SceneComponent.K2_SetRelativeTransform` (`CameraActor.CameraComponent` _returnvalue) (`KismetMathLibrary.MakeTransform` (-0.043341 -0.514562 0.0) (struct :`Yaw` 80.0 :`Roll` -90.0) (0.01 0.01 0.01)) false false)
  (`CameraComponent.SetConstraintAspectRatio` (`CameraActor.CameraComponent` (`local.LocalCamera`)) false)
  (bind _player (`self.Player`)
    (:`then`
      (`PlayerController.SetViewTargetWithBlend` (`Pawn.GetLocalViewingPlayerController` _player) (`local.LocalCamera`) 0.0 "VTBlend_Linear" 0.0 false))
    (:`else`)))

(fn `UserConstructionScript`)