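; Behavior tree task that triggers the AI monster's screamer on the player.
; On execute, it reads the "Player" blackboard value as a BP_FirstPersonCharacter and disables that character's jumping, movement and look.
; It then calls Screamer on the owning AIC_AIMonsterController and never calls Finish Execute.
; A debug print shows the controlled pawn's name.
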(event `self.ReceiveExecuteAI`
  (params (OwnerController :type "AIController Object Reference") (ControlledPawn :type "Pawn Object Reference"))
  (`KismetSystemLibrary.PrintString` (`KismetSystemLibrary.GetDisplayName` ControlledPawn))
  (bind _asbp_first_person_character (cast `/Game/Assets/Blueprints/Player/BP_FirstPersonCharacter` (`BlackboardComponent.GetValueAsObject` (`AIBlueprintHelperLibrary.GetBlackboard` ControlledPawn) "Player")))
  (set `SilenceCharacter.bCanJump` false _asbp_first_person_character)
  (set `SilenceCharacter.bCanMove` false _asbp_first_person_character)
  (set `SilenceCharacter.bCanLook` false _asbp_first_person_character)
  (bind _asaic_aimonster_controller (cast `/Game/Assets/Blueprints/AI/AIC_AIMonsterController` OwnerController))
  (`/Game/Assets/Blueprints/AI/AIC_AIMonsterController.Screamer` _asaic_aimonster_controller))