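; BP_AIMonster is an AI monster Blueprint that screams when its detection animation is triggered.
; PlayScream plays the detect-player montage, disables movement and reports a noise event at the monster's location, then restores walking when the montage completes.
; EnableScreamAssets reveals the spotlight and clears all widgets from the screen.
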(event `EnableScreamAssets`
  (bind _spotlight (`self.SpotLight`))
  (`SceneComponent.SetHiddenInGame` _spotlight false false)
  (`SceneComponent.SetVisibility` _spotlight true false)
  (`WidgetLayoutLibrary.RemoveAllWidgets`))

(event `PlayScream`
  (bind _charactermovement (`self.CharacterMovement`))
  (`|PlayMontage` (`self.Mesh`) (`self.DetectPlayerAnim`)
    (:`then`
      (`CharacterMovementComponent.DisableMovement` _charactermovement)
      (`AISense_Hearing.ReportNoiseEvent` (`self.K2_GetActorLocation`) 1.0 self 1000.0))
    (:`OnCompleted`
      (`CharacterMovementComponent.SetMovementMode` _charactermovement "MOVE_Walking" 0))))

(fn `UserConstructionScript`)