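; Behavior tree service that decides, on activation, whether the AI can attack the player or instead starts a hiding-spot minigame.
; If the Blackboard's Player is within close range and not hidden, it sets CanAttack.
; If the player is hidden in a BP_Cachette not already in game, it calls that actor's heart game, clears CanAttack, sets LaunchGame and writes the AI socket location to Loc.
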(event `self.ReceiveActivationAI`
  (params (OwnerController :type "AIController Object Reference") (ControlledPawn :type "Pawn Object Reference"))
  (bind _returnvalue (`BlackboardComponent.GetValueAsObject` (`AIBlueprintHelperLibrary.GetBlackboard` OwnerController) "Player"))
  (`/Engine/EditorBlueprintResources/StandardMacros.IsValid` _returnvalue
    (:`Is Valid`
      (bind _asbp_first_person_character (cast `/Game/Assets/Blueprints/Player/BP_FirstPersonCharacter` _returnvalue))
      (if (<= (`KismetMathLibrary.Vector_Distance` (`Actor.K2_GetActorLocation` ControlledPawn) (`Actor.K2_GetActorLocation` _asbp_first_person_character)) 150.0)
        (if (not (`/Game/Assets/Blueprints/Player/BP_FirstPersonCharacter.IsInCachette` _asbp_first_person_character))
          (`BTFunctionLibrary.SetBlackboardValueAsBool` (`self.CanAttack`) true)
          (else
            (bind _actorinteract (`/Game/Assets/Blueprints/Player/BP_FirstPersonCharacter.ActorInteract` _asbp_first_person_character)
              (:`then`
                (bind _asbp_cachette (cast `/Game/Assets/Blueprints/Gameplay/BP_Cachette` _actorinteract))
                (if (not (`/Game/Assets/Blueprints/Gameplay/BP_Cachette.bIsInGame` _asbp_cachette))
                  (`/Game/Assets/Blueprints/Gameplay/BP_Cachette.CallHeartGame` _asbp_cachette)
                  (`BTFunctionLibrary.SetBlackboardValueAsBool` (`self.CanAttack`))
                  (`BTFunctionLibrary.SetBlackboardValueAsBool` (`self.LaunchGame`) true)
                  (`BTFunctionLibrary.SetBlackboardValueAsVector` (`self.Loc`) (`SceneComponent.K2_GetComponentLocation` (`/Game/Assets/Blueprints/Gameplay/BP_Cachette.AISocket` _asbp_cachette)))))
              (:`else`))))))))