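; Player controller for the main menu that sets up the menu view and UI and drives a microphone level meter in the options screen.
; On BeginPlay it blends the view to a camera actor found in the level, waits for the blend, then shows the main menu widget with UI-only input and a cursor.
; AudioCapture envelope values are converted to a log scale, remapped, scaled by MicSensibility and fed to the options widget's progress bar.
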(event `self.ReceiveBeginPlay`
  (bind _returnvalue (`GameplayStatics.GetActorOfClass` "/Script/Engine.CameraActor"))
  (`self.SetViewTargetWithBlend` _returnvalue 2.0)
  (`KismetSystemLibrary.Delay` 2.0)
  (bind _returnvalue_2 (`|CreateWidget` "/Game/Assets/Blueprints/UI/UW_MainMenu.UW_MainMenu_C" self))
  (bind _output_get (set `self.MainMenu` _returnvalue_2))
  (`UserWidget.SetOwningPlayer` _output_get self)
  (`UserWidget.AddToViewport` _output_get 0)
  (`WidgetBlueprintLibrary.SetInputMode_UIOnlyEx` self _output_get "LockInFullscreen" true)
  (set `self.bShowMouseCursor` true))

(event `self.AudioCapture.OnAudioEnvelopeValue`
  (params (EnvelopeValue :type "Float (single-precision)"))
  (bind _mainmenu (`self.MainMenu`)
    (:`then`
      (bind _uw_options (`/Game/Assets/Blueprints/UI/UW_MainMenu.UW_Options` _mainmenu)
        (:`then`
          (bind _p_soundplayer (`/Game/Assets/Blueprints/UI/UW_Options.P_SoundPlayer` _uw_options)
            (:`then`
              (`ProgressBar.SetPercent` _p_soundplayer (* (`KismetMathLibrary.MapRangeClamped` (`KismetMathLibrary.Log` EnvelopeValue 10.0) -2.7 -0.7 0.0 1.0) (`self.MicSensibility`))))
            (:`else`)))
        (:`else`)))
    (:`else`)))

(fn `UserConstructionScript`)