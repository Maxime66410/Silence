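; PC_Credit is the player controller for the credits screen, showing the credits widget and providing a way back to the main menu.
; On BeginPlay it creates UW_Credit, adds it to the viewport, shows the cursor and switches to UI-only input with the mouse locked in fullscreen.
; After a short delay it gives the widget focus again.
; An AnyKey press handler opens MAP_MainMenu.
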(event `self.ReceiveBeginPlay`
  (bind _hud (`self.HUD`))
  (bind _returnvalue (`|CreateWidget` "/Game/Assets/Blueprints/UI/UW_Credit.UW_Credit_C" self))
  (bind _output_get (set `self.HUD` _returnvalue))
  (`UserWidget.AddToViewport` _output_get 0)
  (set `self.bShowMouseCursor` true)
  (`WidgetBlueprintLibrary.SetInputMode_UIOnlyEx` self _hud "LockInFullscreen" true)
  (`KismetSystemLibrary.Delay` 0.5)
  (`Widget.SetKeyboardFocus` _hud)
  (`Widget.SetFocus` _hud))

(event `Key|AnyKey`
  (params (Key :type "Key Structure"))
  (:`Pressed`
    (`GameplayStatics.OpenLevelBySoftObjectPtr` "/Game/Assets/Map/MAP_MainMenu.MAP_MainMenu")))

(fn `UserConstructionScript`)