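; BP_Heart is a heart actor for the heart minigame that flies to a target Location and adjusts the game's percent on arrival.
; After short startup delays it picks a left or right mesh from the Right flag and enables Tick.
; Tick moves it at constant speed; on arrival it stops ticking, passes a small negative change to HeartGame, refreshes the HUD and destroys itself.
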(event `self.ReceiveBeginPlay`
  (`KismetSystemLibrary.Delay` 0.2)
  (`StaticMeshComponent.SetStaticMesh` (`self.StaticMesh`) (select `bool` (`self.bRight`) :`false` "/Game/Assets/StaticMesh/Heart/HeartRight.HeartRight" :`true` "/Game/Assets/StaticMesh/Heart/HeartLeft.HeartLeft" :!type "StaticMesh Object Reference"))
  (`KismetSystemLibrary.Delay` 0.2)
  (`self.SetActorTickEnabled` true))

(event `self.ReceiveTick`
  (params (DeltaSeconds :type "Float (single-precision)"))
  (bind _returnvalue (`self.K2_GetActorLocation`))
  (bind _location (`self.Location`))
  (`self.K2_SetActorLocation` (`KismetMathLibrary.VInterpTo_Constant` _returnvalue _location DeltaSeconds 100.0))
  (if (== _returnvalue _location :`ErrorTolerance` 1e-05)
    (`self.SetActorTickEnabled` false)
    (bind _heartgame (`self.HeartGame`)
      (:`then`
        (`/Game/Assets/Blueprints/Gameplay/BP_HeartGame.SetPercent` _heartgame -0.05)
        (bind _hudheartgame (`/Game/Assets/Blueprints/Gameplay/BP_HeartGame.HUDHeartGame` _heartgame)
          (:`then`
            (`/Game/Assets/Blueprints/UI/UW_HeartGame.Setpercent` _hudheartgame (`/Game/Assets/Blueprints/Gameplay/BP_HeartGame.Percent` _heartgame))
            (`KismetSystemLibrary.Delay` 0.01)
            (`self.K2_DestroyActor`))
          (:`else`)))
      (:`else`))))

(fn `UserConstructionScript`)