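; BP_HeartGame runs a timing minigame where hits on BP_Heart actors raise a health-style percentage and misses lower it.
; A looping timer spawns linked left/right heart pairs in random patterns for a random number of rounds.
; EnableTrigger briefly opens the capsule's overlap window, then DisableTrigger scores it, updating UW_HeartGame and playing throttled audio.
; EndGame polls until hearts clear, then rolls win or lose weighted by the percentage.
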(event `EnableTrigger`
  (bind _capsule (`self.Capsule`))
  (set `self.IsHit` false)
  (`PrimitiveComponent.SetCollisionResponseToAllChannels` _capsule "ECR_Overlap")
  (`SceneComponent.SetVisibility` _capsule true false)
  (`KismetSystemLibrary.K2_ClearAndInvalidateTimerHandle` (`self.Event_Trigger`))
  (bind _returnvalue (`KismetSystemLibrary.K2_SetTimerDelegate` (`|CreateDelegate` :!event `DisableTrigger`) 0.05))
  (set `self.Event_Trigger` _returnvalue))

(event `DisableTrigger`
  (bind _capsule (`self.Capsule`))
  (bind _ishit (`self.IsHit`))
  (`KismetSystemLibrary.K2_ClearAndInvalidateTimerHandle` (`self.Event_Trigger`))
  (`KismetSystemLibrary.PrintString` (select `bool` _ishit :`false` "NotHit" :`true` "Hit"))
  (`self.PlayAudio` (select `bool` _ishit :`false` "/Game/Assets/Audio/Bone/SC_Bone_Break.SC_Bone_Break" :`true` "/Game/Assets/Audio/Heart/SC_Heartbeat.SC_Heartbeat" :!type "SoundBase Object Reference"))
  (`self.SetPercent` (select `bool` _ishit :`false` -0.01 :`true` 0.05))
  (bind _hudheartgame (`self.HUDHeartGame`)
    (:`then`
      (`/Game/Assets/Blueprints/UI/UW_HeartGame.Setpercent` _hudheartgame (`self.Percent`)))
    (:`else`
      _))
  (`PrimitiveComponent.SetCollisionResponseToAllChannels` _capsule "ECR_Ignore")
  (`SceneComponent.SetVisibility` _capsule false false))

(event `self.Capsule.OnComponentBeginOverlap`
  (params (OverlappedComponent :type "PrimitiveComponent Object Reference") (OtherActor :type "Actor Object Reference") (OtherComp :type "PrimitiveComponent Object Reference") (OtherBodyIndex :type Integer) (bFromSweep :type Boolean) (SweepResult :type "HitResult Structure (by ref)"))
  (bind _asbp_heart (cast `/Game/Assets/Blueprints/Gameplay/BP_Heart` OtherActor))
  (`/Game/Assets/Blueprints/Gameplay/BP_Heart.CallDestroyParent` _asbp_heart)
  (`self.K2_DestroyActor` _asbp_heart)
  (set `self.IsHit` true)
  (`self.DisableTrigger`))

(event `self.ReceiveBeginPlay`
  ;[1 1 1] BeginPlay
  (`self.InitGame`))

(event `InitGame`
  ;[1 1 1] Init Game
  (bind _returnvalue (`|CreateWidget` "/Game/Assets/Blueprints/UI/UW_HeartGame.UW_HeartGame_C" (`GameplayStatics.GetPlayerController` 0)))
  (set `self.HUDHeartGame` _returnvalue))

(event `StartGame`
  ;[1 1 1] Start Game
  (`self.SetPercent` 1.0)
  (bind _hudheartgame (`self.HUDHeartGame`)
    (:`then`
      (`/Game/Assets/Blueprints/UI/UW_HeartGame.Setpercent` _hudheartgame (`self.Percent`))
      (bind _hudheartgame_2 (`self.HUDHeartGame`)
        (:`then`
          (`UserWidget.AddToViewport` _hudheartgame_2 0)
          (set `self.RoundMax` (`KismetMathLibrary.RandomIntegerInRange` 4 20))
          (set `self.Round` 0)
          (set `self.Time` (`KismetMathLibrary.RandomFloatInRange` 3.0 8.0))
          (bind _returnvalue (`KismetSystemLibrary.K2_SetTimerDelegate` (`|CreateDelegate` :!event `SpawnHeartTime`) (`self.Time`) true))
          (set `self.Event_GameState` _returnvalue)
          (`self.CleanHeartArray`))
        (:`else`)))
    (:`else`)))

(event `SpawnHeartSystem`
  (bind _returnvalue (`SceneComponent.K2_GetComponentLocation` (`self.MainBaseHeart`)))
  (bind _returnvalue_2 (`SceneComponent.K2_GetComponentLocation` (`self.MainBaseHeart`)))
  (bind _returnvalue_3 (`SceneComponent.K2_GetComponentLocation` (`self.MainBaseHeart`)))
  (bind _returnvalue_4 (`SceneComponent.K2_GetComponentLocation` (`self.MainBaseHeart`)))
  (bind _returnvalue_5 (`SceneComponent.K2_GetComponentLocation` (`self.MainBaseHeart`)))
  (bind _returnvalue_6 (`SceneComponent.K2_GetComponentLocation` (`self.MainBaseHeart`)))
  (bind _returnvalue_7 (`SceneComponent.K2_GetComponentLocation` (`self.MainBaseHeart`)))
  ;[1 1 1] Pattern
  (switch `int` (`KismetMathLibrary.RandomInteger` 3)
    (:`0`
      (bind _returnvalue_8 (`|SpawnActorFromClass` "/Game/Assets/Blueprints/Gameplay/BP_Heart.BP_Heart_C" (`KismetMathLibrary.MakeTransform` (`SceneComponent.K2_GetComponentLocation` (`self.PointA`))) "Undefined" "MultiplyWithRoot" null false _returnvalue_4 self null))
      (`KismetArrayLibrary.Array_Add` (`self.HeartArray`) _returnvalue_8)
      (bind _returnvalue_9 (`|SpawnActorFromClass` "/Game/Assets/Blueprints/Gameplay/BP_Heart.BP_Heart_C" (`KismetMathLibrary.MakeTransform` (`SceneComponent.K2_GetComponentLocation` (`self.PointB`))) "Undefined" "MultiplyWithRoot" null true _returnvalue_4 self null))
      (`KismetArrayLibrary.Array_Add` (`self.HeartArray`) _returnvalue_9)
      (set `/Game/Assets/Blueprints/Gameplay/BP_Heart.HeartParent` _returnvalue_9 _returnvalue_8)
      (set `/Game/Assets/Blueprints/Gameplay/BP_Heart.HeartParent` _returnvalue_8 _returnvalue_9)
      (`KismetSystemLibrary.Delay` 1.5)
      (bind _returnvalue_10 (`|SpawnActorFromClass` "/Game/Assets/Blueprints/Gameplay/BP_Heart.BP_Heart_C" (`KismetMathLibrary.MakeTransform` (`SceneComponent.K2_GetComponentLocation` (`self.PointA`))) "Undefined" "MultiplyWithRoot" null false _returnvalue_5 self null))
      (`KismetArrayLibrary.Array_Add` (`self.HeartArray`) _returnvalue_10)
      (bind _returnvalue_11 (`|SpawnActorFromClass` "/Game/Assets/Blueprints/Gameplay/BP_Heart.BP_Heart_C" (`KismetMathLibrary.MakeTransform` (`SceneComponent.K2_GetComponentLocation` (`self.PointB`))) "Undefined" "MultiplyWithRoot" null true _returnvalue_5 self null))
      (`KismetArrayLibrary.Array_Add` (`self.HeartArray`) _returnvalue_11)
      (set `/Game/Assets/Blueprints/Gameplay/BP_Heart.HeartParent` _returnvalue_11 _returnvalue_10)
      (set `/Game/Assets/Blueprints/Gameplay/BP_Heart.HeartParent` _returnvalue_10 _returnvalue_11))
    (:`1`
      (bind _returnvalue_12 (`|SpawnActorFromClass` "/Game/Assets/Blueprints/Gameplay/BP_Heart.BP_Heart_C" (`KismetMathLibrary.MakeTransform` (`SceneComponent.K2_GetComponentLocation` (`self.PointA`))) "Undefined" "MultiplyWithRoot" null false _returnvalue_6 self null))
      (`KismetArrayLibrary.Array_Add` (`self.HeartArray`) _returnvalue_12)
      (bind _returnvalue_13 (`|SpawnActorFromClass` "/Game/Assets/Blueprints/Gameplay/BP_Heart.BP_Heart_C" (`KismetMathLibrary.MakeTransform` (`SceneComponent.K2_GetComponentLocation` (`self.PointB`))) "Undefined" "MultiplyWithRoot" null true _returnvalue_6 self null))
      (`KismetArrayLibrary.Array_Add` (`self.HeartArray`) _returnvalue_13)
      (set `/Game/Assets/Blueprints/Gameplay/BP_Heart.HeartParent` _returnvalue_13 _returnvalue_12)
      (set `/Game/Assets/Blueprints/Gameplay/BP_Heart.HeartParent` _returnvalue_12 _returnvalue_13)
      (`KismetSystemLibrary.Delay` 1.0)
      (bind _returnvalue_14 (`|SpawnActorFromClass` "/Game/Assets/Blueprints/Gameplay/BP_Heart.BP_Heart_C" (`KismetMathLibrary.MakeTransform` (`SceneComponent.K2_GetComponentLocation` (`self.PointA`))) "Undefined" "MultiplyWithRoot" null false _returnvalue_7 self null))
      (`KismetArrayLibrary.Array_Add` (`self.HeartArray`) _returnvalue_14)
      (bind _returnvalue_15 (`|SpawnActorFromClass` "/Game/Assets/Blueprints/Gameplay/BP_Heart.BP_Heart_C" (`KismetMathLibrary.MakeTransform` (`SceneComponent.K2_GetComponentLocation` (`self.PointB`))) "Undefined" "MultiplyWithRoot" null true _returnvalue_7 self null))
      (`KismetArrayLibrary.Array_Add` (`self.HeartArray`) _returnvalue_15)
      (set `/Game/Assets/Blueprints/Gameplay/BP_Heart.HeartParent` _returnvalue_15 _returnvalue_14)
      (set `/Game/Assets/Blueprints/Gameplay/BP_Heart.HeartParent` _returnvalue_14 _returnvalue_15))
    (:`2`
      (bind _returnvalue_16 (`|SpawnActorFromClass` "/Game/Assets/Blueprints/Gameplay/BP_Heart.BP_Heart_C" (`KismetMathLibrary.MakeTransform` (`SceneComponent.K2_GetComponentLocation` (`self.PointA`))) "Undefined" "MultiplyWithRoot" null false _returnvalue_3 self null))
      (`KismetArrayLibrary.Array_Add` (`self.HeartArray`) _returnvalue_16)
      (bind _returnvalue_17 (`|SpawnActorFromClass` "/Game/Assets/Blueprints/Gameplay/BP_Heart.BP_Heart_C" (`KismetMathLibrary.MakeTransform` (`SceneComponent.K2_GetComponentLocation` (`self.PointB`))) "Undefined" "MultiplyWithRoot" null true _returnvalue_3 self null))
      (`KismetArrayLibrary.Array_Add` (`self.HeartArray`) _returnvalue_17)
      (set `/Game/Assets/Blueprints/Gameplay/BP_Heart.HeartParent` _returnvalue_17 _returnvalue_16)
      (set `/Game/Assets/Blueprints/Gameplay/BP_Heart.HeartParent` _returnvalue_16 _returnvalue_17)
      (`KismetSystemLibrary.Delay` 1.0)
      (bind _returnvalue_18 (`|SpawnActorFromClass` "/Game/Assets/Blueprints/Gameplay/BP_Heart.BP_Heart_C" (`KismetMathLibrary.MakeTransform` (`SceneComponent.K2_GetComponentLocation` (`self.PointA`))) "Undefined" "MultiplyWithRoot" null false _returnvalue self null))
      (`KismetArrayLibrary.Array_Add` (`self.HeartArray`) _returnvalue_18)
      (bind _returnvalue_19 (`|SpawnActorFromClass` "/Game/Assets/Blueprints/Gameplay/BP_Heart.BP_Heart_C" (`KismetMathLibrary.MakeTransform` (`SceneComponent.K2_GetComponentLocation` (`self.PointB`))) "Undefined" "MultiplyWithRoot" null true _returnvalue self null))
      (`KismetArrayLibrary.Array_Add` (`self.HeartArray`) _returnvalue_19)
      (set `/Game/Assets/Blueprints/Gameplay/BP_Heart.HeartParent` _returnvalue_19 _returnvalue_18)
      (set `/Game/Assets/Blueprints/Gameplay/BP_Heart.HeartParent` _returnvalue_18 _returnvalue_19)
      (`KismetSystemLibrary.Delay` 1.0)
      (bind _returnvalue_20 (`|SpawnActorFromClass` "/Game/Assets/Blueprints/Gameplay/BP_Heart.BP_Heart_C" (`KismetMathLibrary.MakeTransform` (`SceneComponent.K2_GetComponentLocation` (`self.PointA`))) "Undefined" "MultiplyWithRoot" null false _returnvalue_2 self null))
      (`KismetArrayLibrary.Array_Add` (`self.HeartArray`) _returnvalue_20)
      (bind _returnvalue_21 (`|SpawnActorFromClass` "/Game/Assets/Blueprints/Gameplay/BP_Heart.BP_Heart_C" (`KismetMathLibrary.MakeTransform` (`SceneComponent.K2_GetComponentLocation` (`self.PointB`))) "Undefined" "MultiplyWithRoot" null true _returnvalue_2 self null))
      (`KismetArrayLibrary.Array_Add` (`self.HeartArray`) _returnvalue_21)
      (set `/Game/Assets/Blueprints/Gameplay/BP_Heart.HeartParent` _returnvalue_21 _returnvalue_20)
      (set `/Game/Assets/Blueprints/Gameplay/BP_Heart.HeartParent` _returnvalue_20 _returnvalue_21))))

(event `SpawnHeartTime`
  ;[1 1 1] Game State
  (`/Engine/EditorBlueprintResources/StandardMacros.IncrementInt` (`self.Round`)
    (:`  `
      (`self.SpawnHeartSystem`)
      (if (>= (`self.Round`) (`self.RoundMax`))
        (`KismetSystemLibrary.K2_ClearAndInvalidateTimerHandle` (`self.Event_GameState`))
        (`self.EndGame`)))))

(event `EndGame`
  ;[1 1 1] EndGame
  (if (`KismetArrayLibrary.Array_IsEmpty` (`self.HeartArray`))
    (if (`KismetMathLibrary.RandomBoolWithWeight` (`self.Percent`))
      (`KismetSystemLibrary.PrintString` "Win")
      (else
        (`KismetSystemLibrary.PrintString` "Loose")))
    (bind _hudheartgame (`self.HUDHeartGame`)
      (:`then`
        (`Widget.RemoveFromParent` _hudheartgame))
      (:`else`))
    (else
      (`self.CheckClearHeart`)
      (`KismetSystemLibrary.K2_SetTimerDelegate` (`|CreateDelegate` :!event `EndGame`) 1.0))))

(event `PlayAudio`
  (params (Sound :type "SoundBase Object Reference"))
  (`/Engine/EditorBlueprintResources/StandardMacros.DoOnce` false :!label _label
    (:`Completed`
      (`GameplayStatics.PlaySound2D` Sound 1.0 1.0 0.0 null null)
      (`KismetSystemLibrary.K2_SetTimerDelegate` (delegate `PlayAudioReset`) 0.04))))

(event `PlayAudioReset`
  (goto _label :!via `Reset`))

(fn `CheckClearHeart`
  (locals (NewArray :type "Array of /Game/Assets/Blueprints/Gameplay/BP_Heart Object Reference"))
  (for _array_element (`self.HeartArray`)
    (`/Engine/EditorBlueprintResources/StandardMacros.IsValid` _array_element
      (:`Is Valid`
        (`KismetArrayLibrary.Array_Add` (`local.NewArray`) _array_element))))
  (set `self.HeartArray` (`local.NewArray`)))

(fn `CleanHeartArray`
  (bind _heartarray (`self.HeartArray`))
  (for _array_element _heartarray
    (`self.K2_DestroyActor` _array_element))
  (`KismetArrayLibrary.Array_Clear` _heartarray))

(fn `SetPercent`
  (params (B :type "Float (double-precision)"))
  (set `self.Percent` (`KismetMathLibrary.FClamp` (+ (`self.Percent`) B))))

(fn `UserConstructionScript`)