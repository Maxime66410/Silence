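; Cabinet hiding spot (cachette) the player can enter and leave, with an optional linked HeartGame minigame.
; Fire and Cancel toggle the character's movement, look and flashlight, while timelines swing four doors and lerp the player between saved transform and cabinet socket.
; Door sounds also report AI-audible noise at AISocket.
; A debug box, disabled while hiding, teleports overlapping players to AISocket.
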(event `self.ReceiveBeginPlay`
  ;[0 0 0] Init
  (`TimelineComponent.SetPlayRate` (`self.ForcePlayerOnTarget`) 1.0)
  (`TimelineComponent.SetPlayRate` (`self.DoorTimeLine`) 2.0))

(event `Call_ForcePlayerOnTarget`
  (params (BEnter :type Boolean))
  (bind (_returnvalue_location _returnvalue_rotation) (`KismetMathLibrary.BreakTransform` (`SceneComponent.K2_GetComponentToWorld` (`self.CabinetSocket`))))
  ;[1 1 1] TargetPlayer
  (if BEnter
    (bind (_direction _move) (`Timeline|ForcePlayerOnTarget` :!label _label)
      (:`Update`
        (bind _as_bp_first_person_character (`self.As BP First Person Character`)
          (:`then`
            (`self.K2_SetActorLocation` _as_bp_first_person_character (`KismetMathLibrary.VLerp` (`self.PlrLoc`) _returnvalue_location _move) false false)
            (bind _returnvalue (`KismetMathLibrary.RLerp` (`self.PlrRot`) _returnvalue_rotation _move))
            (`self.K2_SetActorRotation` _as_bp_first_person_character _returnvalue false)
            (`Controller.SetControlRotation` (`Pawn.GetController` _as_bp_first_person_character) _returnvalue))
          (:`else`)))
      (:`Finished`
        (`self.Call_DoorAnimation` false)
        (if (not BEnter)
          (`self.CollisionDebugTest` false))))
    (else
      (goto _label :!via `Reverse`))))

(event `CallHeartGame`
  (bind _heartgame (`self.HeartGame`)
    (:`then`
      (set `/Game/Assets/Blueprints/Gameplay/BP_HeartGame.LastCachette` self _heartgame)
      (`/Game/Assets/Blueprints/Gameplay/BP_HeartGame.StartGame` _heartgame)
      (set `self.bIsInGame` true)
      (bind _as_bp_first_person_character (`self.As BP First Person Character`)
        (:`then`
          (set `self.PlrLoc` (`self.K2_GetActorLocation` _as_bp_first_person_character))
          (set `self.PlrRot` (`self.K2_GetActorRotation` _as_bp_first_person_character))
          (set `self.PlrControlRot` (`Pawn.GetControlRotation` _as_bp_first_person_character))
          (set `SilenceCharacter.bCanMove` false _as_bp_first_person_character)
          (set `SilenceCharacter.bCanJump` false _as_bp_first_person_character)
          (set `SilenceCharacter.bCanLook` false _as_bp_first_person_character)
          (set `/Game/Assets/Blueprints/Player/BP_FirstPersonCharacter.IsInCachette` true _as_bp_first_person_character)
          (`/Game/Assets/Blueprints/Player/BP_FirstPersonCharacter.Flash Light Connect` _as_bp_first_person_character false)
          (`self.Call_ForcePlayerOnTarget` true))
        (:`else`)))
    (:`else`)))

(event `Call_DoorAnimation`
  (params (bOpen :type Boolean))
  ;[1 1 1] OpenCloseDoor
  (if bOpen
    (`self.PlaySound` true)
    (bind (_direction _move) (`Timeline|DoorTimeLine` :!label _label_2)
      (:`Update`
        (`SceneComponent.K2_SetRelativeRotation` (`self.SM_Rack_Door`) (`KismetMathLibrary.RLerp` (struct) (struct :`Yaw` 90.0) _move) false false)
        (`SceneComponent.K2_SetRelativeRotation` (`self.SM_Rack_Door1`) (`KismetMathLibrary.RLerp` (struct) (struct :`Yaw` 90.0) _move) false false)
        (`SceneComponent.K2_SetRelativeRotation` (`self.SM_Rack_Door2`) (`KismetMathLibrary.RLerp` (struct) (struct :`Yaw` -90.0) _move) false false)
        (`SceneComponent.K2_SetRelativeRotation` (`self.SM_Rack_Door3`) (`KismetMathLibrary.RLerp` (struct) (struct :`Yaw` -90.0) _move) false false))
      (:`Finished`
        (if (not bOpen)
          (`self.PlaySound` false))))
    (else
      (goto _label_2 :!via `Reverse`))))

(event `/Game/Assets/Blueprints/Interface/BPI_Interact.Fire`
  (params (Plr :type "/Game/Assets/Blueprints/Player/BP_FirstPersonCharacter Object Reference"))
  ;[1 1 1] Enter Cachette
  (set `self.As BP First Person Character` Plr)
  (if (not (`self.bIsInGame`))
    (if (not (`self.bPlayerIsHere`))
      (set `self.bPlayerIsHere` true)
      (`self.Call_DoorAnimation` true)
      (bind _as_bp_first_person_character (`self.As BP First Person Character`)
        (:`then`
          (set `self.PlrLoc` (`self.K2_GetActorLocation` _as_bp_first_person_character))
          (set `self.PlrRot` (`self.K2_GetActorRotation` _as_bp_first_person_character))
          (set `self.PlrControlRot` (`Pawn.GetControlRotation` _as_bp_first_person_character))
          (set `SilenceCharacter.bCanMove` false _as_bp_first_person_character)
          (set `SilenceCharacter.bCanJump` false _as_bp_first_person_character)
          (set `SilenceCharacter.bCanLook` false _as_bp_first_person_character)
          (set `/Game/Assets/Blueprints/Player/BP_FirstPersonCharacter.IsInCachette` true _as_bp_first_person_character)
          (`/Game/Assets/Blueprints/Player/BP_FirstPersonCharacter.Flash Light Connect` _as_bp_first_person_character false)
          (`self.CollisionDebugTest` true)
          (`self.Call_ForcePlayerOnTarget` true))
        (:`else`)))
    (else
      ;;[1 1 1] Play Heart Game
      (bind _heartgame (`self.HeartGame`)
        (:`then`
          (`/Game/Assets/Blueprints/Gameplay/BP_HeartGame.EnableTrigger` _heartgame))
        (:`else`)))))

(event `self.DebugBox.OnComponentBeginOverlap`
  (params (OverlappedComponent :type "PrimitiveComponent Object Reference") (OtherActor :type "Actor Object Reference") (OtherComp :type "PrimitiveComponent Object Reference") (OtherBodyIndex :type Integer) (bFromSweep :type Boolean) (SweepResult :type "HitResult Structure (by ref)"))
  (bind _asbp_first_person_character (cast `/Game/Assets/Blueprints/Player/BP_FirstPersonCharacter` OtherActor))
  (`self.K2_SetActorLocation` _asbp_first_person_character (`SceneComponent.K2_GetComponentLocation` (`self.AISocket`)) false false))

(event `/Game/Assets/Blueprints/Interface/BPI_Interact.Cancel`
  (params (Plr :type "/Game/Assets/Blueprints/Player/BP_FirstPersonCharacter Object Reference"))
  ;[1 1 1] Exit cachette
  (set `self.As BP First Person Character` Plr)
  (if (not (`self.bIsInGame`))
    (if (`self.bPlayerIsHere`)
      (set `self.bPlayerIsHere` false)
      (`self.Call_DoorAnimation` true)
      (`self.Call_ForcePlayerOnTarget` false)
      (`KismetSystemLibrary.RetriggerableDelay` 1.0)
      (bind _as_bp_first_person_character (`self.As BP First Person Character`)
        (:`then`
          (set `SilenceCharacter.bCanMove` true _as_bp_first_person_character)
          (set `SilenceCharacter.bCanJump` true _as_bp_first_person_character)
          (set `SilenceCharacter.bCanLook` true _as_bp_first_person_character)
          (set `/Game/Assets/Blueprints/Player/BP_FirstPersonCharacter.IsInCachette` false _as_bp_first_person_character)
          (`/Game/Assets/Blueprints/Player/BP_FirstPersonCharacter.Flash Light Connect` _as_bp_first_person_character true))
        (:`else`)))))

(fn `CollisionDebugTest`
  (params (bBool :type Boolean))
  (bind _returnvalue (not bBool))
  (bind _debugbox (`self.DebugBox`))
  (`SceneComponent.SetHiddenInGame` _debugbox bBool false)
  (`SceneComponent.SetVisibility` _debugbox _returnvalue false)
  (`PrimitiveComponent.SetCollisionEnabled` (`self.DebugBox`) (select `bool` _returnvalue :`false` "NoCollision" :`true` "QueryOnly" :!type "ECollisionEnabled Enum")))

(fn `PlaySound`
  (params (bIsOpen :type Boolean))
  (`GameplayStatics.PlaySoundAtLocation` (select `bool` bIsOpen :`false` "/Game/Assets/Audio/Environment/Cabinet/SC_CabinetCloseDoor.SC_CabinetCloseDoor" :`true` "/Game/Assets/Audio/Environment/Cabinet/SC_CabinetOpenDoor.SC_CabinetOpenDoor" :!type "SoundBase Object Reference") (`SceneComponent.K2_GetComponentLocation` (`self.CabinetSocket`)) (struct) 1.0 1.0 0.0 null null null null)
  (`AISense_Hearing.ReportNoiseEvent` (`SceneComponent.K2_GetComponentLocation` (`self.AISocket`)) 1.0 self 1000.0))

(fn `UserConstructionScript`)