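; BP_PartGenerator is an actor whose visible behavior is a static mesh spinning around its yaw axis.
; BeginPlay offsets the mesh by RandomRot, then enables actor tick after a short delay.
; Tick adds Speed as local yaw each frame without delta-time scaling, so spin rate follows frame rate.
; A DestroyNOW event destroys the actor, and no part-generation logic appears in its graphs.
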(event `self.ReceiveBeginPlay`
  (`SceneComponent.K2_AddLocalRotation` (`self.StaticMesh`) (`KismetMathLibrary.MakeRotator` 0.0 0.0 (`self.RandomRot`)) false false)
  (`KismetSystemLibrary.Delay` 0.2)
  (`self.SetActorTickEnabled` true))

(event `self.ReceiveTick`
  (params (DeltaSeconds :type "Float (single-precision)"))
  (`SceneComponent.K2_AddLocalRotation` (`self.StaticMesh`) (`KismetMathLibrary.MakeRotator` 0.0 0.0 (`self.Speed`)) false false))

(event `DestroyNOW`
  (`self.K2_DestroyActor`))

(fn `UserConstructionScript`)