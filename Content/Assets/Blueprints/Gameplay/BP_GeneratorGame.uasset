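; Timed skill-check minigame for repairing a generator, with its own HUD and progress read from LastCachette.
; A looping timer spawns randomly paced BP_PartGenerator actors one at a time, and a briefly enabled capsule trigger scores overlaps as hits.
; Hits add progress until three finishes the generator, while misses call ExplodeGenerator on LastCachette.
; LaunchAttack finds the monster nearest the generator and triggers its AI controller's Screamer.
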(event `EnableTrigger`
  (bind _capsule (`self.Capsule`))
  (set `self.IsHit` false)
  (`PrimitiveComponent.SetCollisionResponseToAllChannels` _capsule "ECR_Overlap")
  (`SceneComponent.SetVisibility` _capsule true false)
  (`KismetSystemLibrary.K2_ClearAndInvalidateTimerHandle` (`self.Event_Trigger`))
  (bind _returnvalue (`KismetSystemLibrary.K2_SetTimerDelegate` (`|CreateDelegate` :!event `DisableTrigger`) 0.05))
  (set `self.Event_Trigger` _returnvalue))

(event `DisableTrigger`
  (bind _capsule (`self.Capsule`))
  (bind _ishit (`self.IsHit`))
  (`KismetSystemLibrary.K2_ClearAndInvalidateTimerHandle` (`self.Event_Trigger`))
  (`KismetSystemLibrary.PrintString` (select `bool` _ishit :`false` "NotHit" :`true` "Hit"))
  (`self.PlayAudio` (select `bool` _ishit :`false` "/Game/Assets/Audio/Bone/SC_Bone_Break.SC_Bone_Break" :`true` "/Game/Assets/Audio/Heart/SC_Heartbeat.SC_Heartbeat" :!type "SoundBase Object Reference"))
  (`self.SetPercent` (select `bool` _ishit :`true` 1))
  (`PrimitiveComponent.SetCollisionResponseToAllChannels` _capsule "ECR_Ignore")
  (`SceneComponent.SetVisibility` _capsule false false)
  (if _ishit
    (if (>= (`self.Progress`) 3)
      (`self.EndGame` true))
    (else
      (bind _lastcachette (`self.LastCachette`)
        (:`then`
          (`/Game/Assets/Blueprints/Gameplay/BP_Generator.ExplodeGenerator` _lastcachette))
        (:`else`)))))

(event `self.Capsule.OnComponentBeginOverlap`
  (params (OverlappedComponent :type "PrimitiveComponent Object Reference") (OtherActor :type "Actor Object Reference") (OtherComp :type "PrimitiveComponent Object Reference") (OtherBodyIndex :type Integer) (bFromSweep :type Boolean) (SweepResult :type "HitResult Structure (by ref)"))
  (bind _asbp_part_generator (cast `/Game/Assets/Blueprints/Gameplay/BP_PartGenerator` OtherActor))
  (`self.K2_DestroyActor` _asbp_part_generator)
  (set `self.IsHit` true)
  (`self.DisableTrigger`))

(event `CallExplodeGenerator`
  (bind _lastcachette (`self.LastCachette`)
    (:`then`
      (`/Game/Assets/Blueprints/Gameplay/BP_Generator.ExplodeGenerator` _lastcachette))
    (:`else`)))

(event `self.ReceiveBeginPlay`
  ;[1 1 1] BeginPlay
  (`self.InitGame`))

(event `InitGame`
  ;[1 1 1] Init Game
  (bind _returnvalue (`|CreateWidget` "/Game/Assets/Blueprints/UI/UW_GeneratorGame.UW_GeneratorGame_C" (`GameplayStatics.GetPlayerController` 0)))
  (set `self.HUDGeneratorGame` _returnvalue))

(event `StartGame`
  ;[1 1 1] Start Game
  (bind _hudgeneratorgame (`self.HUDGeneratorGame`)
    (:`then`
      (`UserWidget.AddToViewport` _hudgeneratorgame 0)
      (bind _lastcachette (`self.LastCachette`)
        (:`then`
          (set `self.Progress` (`/Game/Assets/Blueprints/Gameplay/BP_Generator.Progress` _lastcachette))
          (set `self.RoundMax` 1000000)
          (set `self.Round` 0)
          (set `self.Time` (`KismetMathLibrary.RandomFloatInRange` 1.0 4.0))
          (bind _returnvalue (`KismetSystemLibrary.K2_SetTimerDelegate` (`|CreateDelegate` :!event `SpawnHeartTime`) (`self.Time`) true))
          (set `self.Event_GameState` _returnvalue)
          (`self.CleanGeneratorArray`)
          (`GameplayStatics.PlaySound2D` null 1.0 1.0 0.0 null null))
        (:`else`)))
    (:`else`)))

(event `SpawnPartSystem`
  ;[1 1 1] Pattern
  (bind _returnvalue (`|SpawnActorFromClass` "/Game/Assets/Blueprints/Gameplay/BP_PartGenerator.BP_PartGenerator_C" (`KismetMathLibrary.MakeTransform` (`self.K2_GetActorLocation`)) "Undefined" "MultiplyWithRoot" null self (`KismetMathLibrary.RandomFloatInRange` 1.0 3.0) null))
  (set `self.LastPart` _returnvalue)
  (`KismetArrayLibrary.Array_Add` (`self.GeneratorArray`) _returnvalue))

(event `SpawnHeartTime`
  ;[1 1 1] Game State
  (`self.LastPart`
    (:`then`)
    (:`else`
      (if (>= (`self.Progress`) 3)
        (`KismetSystemLibrary.K2_ClearAndInvalidateTimerHandle` (`self.Event_GameState`) :!label _label)
        (`self.EndGame` false)
        (else
          (`/Engine/EditorBlueprintResources/StandardMacros.IncrementInt` (`self.Round`)
            (:`  `
              (`self.SpawnPartSystem`)
              (if (>= (`self.Round`) (`self.RoundMax`))
                (goto _label)))))))))

(event `EndGame`
  (params (bForced :type Boolean))
  ;[1 1 1] EndGame
  (if bForced
    (`self.CleanGeneratorArray`))
  (if (`KismetArrayLibrary.Array_IsEmpty` (`self.GeneratorArray`))
    (if (>= (`self.Progress`) 3)
      (bind _lastcachette (`self.LastCachette`)
        (:`then`
          (`/Game/Assets/Blueprints/Gameplay/BP_Generator.Finish` _lastcachette))
        (:`else`))
      (else
        (bind _lastcachette_2 (`self.LastCachette`)
          (:`then`
            (`/Game/Assets/Blueprints/Interface/BPI_Interact.Cancel` _lastcachette_2 (`/Game/Assets/Blueprints/Gameplay/BP_Generator.As BP First Person Character` _lastcachette_2))
            (set `/Game/Assets/Blueprints/Gameplay/BP_Generator.Progress` (`self.Progress`) _lastcachette_2))
          (:`else`))))
    (bind _hudgeneratorgame (`self.HUDGeneratorGame`)
      (:`then`
        (`Widget.RemoveFromParent` _hudgeneratorgame))
      (:`else`))
    (else
      (`self.CheckClearGenerator`)
      (`KismetSystemLibrary.K2_SetTimerDelegate` (`|CreateDelegate` :!event `EndGameCall`) 1.0))))

(event `EndGameCall`
  ;[1 1 1] EndGame
  (`self.EndGame` false))

(event `PlayAudio`
  (params (Sound :type "SoundBase Object Reference"))
  (`/Engine/EditorBlueprintResources/StandardMacros.DoOnce` false :!label _label
    (:`Completed`
      (`GameplayStatics.PlaySound2D` Sound 1.0 1.0 0.0 null null)
      (`KismetSystemLibrary.K2_SetTimerDelegate` (delegate `PlayAudioReset`) 0.04))))

(event `PlayAudioReset`
  (goto _label :!via `Reset`))

(fn `CheckClearGenerator`
  (locals (NewArray :type "Array of /Game/Assets/Blueprints/Gameplay/BP_PartGenerator Object Reference"))
  (for _array_element (`self.GeneratorArray`)
    (`/Engine/EditorBlueprintResources/StandardMacros.IsValid` _array_element
      (:`Is Valid`
        (`KismetArrayLibrary.Array_Add` (`local.NewArray`) _array_element))))
  (set `self.GeneratorArray` (`local.NewArray`)))

(fn `CleanGeneratorArray`
  (bind _generatorarray (`self.GeneratorArray`))
  (for _array_element _generatorarray
    (`/Engine/EditorBlueprintResources/StandardMacros.IsValid` _array_element
      (:`Is Valid`
        (`self.K2_DestroyActor` _array_element))))
  (`KismetArrayLibrary.Array_Clear` _generatorarray))

(fn `LaunchAttack`
  (locals (ArrayMonster :type "Array of /Game/Assets/Blueprints/AI/BP_AIMonster Object Reference") (MapMonster :type "Map of Float (double-precision) to /Game/Assets/Blueprints/AI/BP_AIMonster Object Reference") (ClosestDistance :type "Float (double-precision)") (ClosestIndex :type Integer))
  (bind (_value _returnvalue) (`BlueprintMapLibrary.Map_Find` (`local.MapMonster`) (`local.ClosestDistance`)))
  (bind _outactors (`GameplayStatics.GetAllActorsOfClass` "/Game/Assets/Blueprints/AI/BP_AIMonster.BP_AIMonster_C"))
  (bind _output_get (set `local.ArrayMonster` _outactors))
  (for _array_element _output_get
    (bind _lastcachette (`self.LastCachette`)
      (:`then`
        (`BlueprintMapLibrary.Map_Add` (`local.MapMonster`) (`KismetMathLibrary.Vector_Distance` (`self.K2_GetActorLocation` _array_element) (`self.K2_GetActorLocation` _lastcachette)) _array_element))
      (:`else`)))
  (bind _keys (`BlueprintMapLibrary.Map_Keys` (`local.MapMonster`)))
  (for (_array_element_2 _array_index) _keys
    (if (== _array_index 0)
      (set `local.ClosestDistance` _array_element_2)
      (set `local.ClosestIndex` 0)
      (elif (> (`local.ClosestDistance`) _array_element_2)
        (set `local.ClosestDistance` _array_element_2)
        (set `local.ClosestIndex` _array_index))))
  (if _returnvalue
    (bind _asaic_aimonster_controller (cast `/Game/Assets/Blueprints/AI/AIC_AIMonsterController` (`AIBlueprintHelperLibrary.GetAIController` _value)))
    (`/Game/Assets/Blueprints/AI/AIC_AIMonsterController.Screamer` _asaic_aimonster_controller)))

(fn `SetPercent`
  (params (B :type Integer))
  (set `self.Progress` (+ (`self.Progress`) B)))

(fn `UserConstructionScript`)