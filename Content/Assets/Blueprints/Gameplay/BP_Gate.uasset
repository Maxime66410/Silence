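; BP_Gate is the level exit gate that opens once enough generators check in and ends the game when the player reaches it.
; It counts AddOpenCheck calls against the generator array's length, filled from all BP_Generator actors if empty.
; Opening swings both doors on a timeline, plays sound, turns lights green and reports long-range AI noise.
; A one-shot box overlap freezes the player, destroys all monsters and calls EndUI.
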(event `self.ReceiveBeginPlay`
  (if (not (`KismetArrayLibrary.Array_IsNotEmpty` (`self.ArrayGenerator`)))
    (`self.GetAllGenerator`))
  (set `self.ToOpen` (`KismetArrayLibrary.Array_Length` (`self.ArrayGenerator`))))

(event `CallOpenDoor`
  (if (not (`self.IsOpen`))
    (set `self.IsOpen` true)
    (`GameplayStatics.PlaySoundAtLocation` "/Game/Assets/Audio/Environment/Door/OpenDoor.OpenDoor" (`self.K2_GetActorLocation`) (struct) 1.0 1.0 0.0 "/Game/Assets/Audio/Attenuation/SA_VeryLoud.SA_VeryLoud" null null null)
    (`AISense_Hearing.ReportNoiseEvent` (`SceneComponent.K2_GetComponentLocation` (`self.AITarget`)) 1.0 self 100000.0)
    (`self.FeedbackEnv`)
    (bind (_direction _move) (`Timeline|OpenDoor`)
      (:`Update`
        (`SceneComponent.K2_SetRelativeRotation` (`self.DoorLeft`) (`KismetMathLibrary.RLerp` (struct) (struct :`Yaw` 90.0) _move) false false)
        (`SceneComponent.K2_SetRelativeRotation` (`self.DoorRight`) (`KismetMathLibrary.RLerp` (struct) (struct :`Yaw` -90.0) _move) false false)))))

(event `AddOpenCheck`
  (`/Engine/EditorBlueprintResources/StandardMacros.IncrementInt` (`self.CurrentToOpen`)
    (:`  `
      (if (>= (`self.CurrentToOpen`) (`self.ToOpen`))
        (`self.CallOpenDoor`)))))

(event `self.Box.OnComponentBeginOverlap`
  (params (OverlappedComponent :type "PrimitiveComponent Object Reference") (OtherActor :type "Actor Object Reference") (OtherComp :type "PrimitiveComponent Object Reference") (OtherBodyIndex :type Integer) (bFromSweep :type Boolean) (SweepResult :type "HitResult Structure (by ref)"))
  (bind _asbp_first_person_character (cast `/Game/Assets/Blueprints/Player/BP_FirstPersonCharacter` OtherActor))
  (`/Engine/EditorBlueprintResources/StandardMacros.DoOnce` false
    (:`Completed`
      (set `SilenceCharacter.bCanMove` false _asbp_first_person_character)
      (set `SilenceCharacter.bCanJump` false _asbp_first_person_character)
      (set `SilenceCharacter.bCanLook` false _asbp_first_person_character)
      (`self.ClearAllAI`)
      (bind _aspc_first_person_player_controller (cast `/Game/Assets/Blueprints/Player/PC_FirstPersonPlayerController` (`GameplayStatics.GetPlayerController` 0)))
      (`/Game/Assets/Blueprints/Player/PC_FirstPersonPlayerController.EndUI` _aspc_first_person_player_controller))))

(fn `ClearAllAI`
  (bind _outactors (`GameplayStatics.GetAllActorsOfClass` "/Game/Assets/Blueprints/AI/BP_AIMonster.BP_AIMonster_C"))
  (for _array_element _outactors
    (`/Engine/EditorBlueprintResources/StandardMacros.IsValid` _array_element
      (:`Is Valid`
        (`self.K2_DestroyActor` _array_element)))))

(fn `FeedbackEnv`
  (`PrimitiveComponent.SetMaterial` (`self.StaticMesh`) 0 "/Game/Hospital_Meshingun/Environment/Asset/Material/props/MI_ExitPanel_01c.MI_ExitPanel_01c")
  (`LightComponent.SetLightColor` (`self.RectLight`) (struct :`R` 0.062745 :`G` 1.0 :`A` 1.0) true)
  (`LightComponent.SetLightColor` (`self.RectLight1`) (struct :`R` 0.062745 :`G` 1.0 :`A` 1.0) true)
  (`PrimitiveComponent.SetMaterial` (`self.StaticMesh1`) 0 "/Game/Assets/Materials/M_Cable01.M_Cable01"))

(fn `GetAllGenerator`
  (`KismetArrayLibrary.Array_Clear` (`self.ArrayGenerator`))
  (bind _outactors (`GameplayStatics.GetAllActorsOfClass` "/Game/Assets/Blueprints/Gameplay/BP_Generator.BP_Generator_C"))
  (set `self.ArrayGenerator` _outactors))

(fn `UserConstructionScript`)