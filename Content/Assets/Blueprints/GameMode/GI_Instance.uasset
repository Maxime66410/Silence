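; Game instance that loads, holds and persists player settings: microphone and mouse sensitivity, DGI and RM methods, and master audio.
; Init loads the SG_DataGame save from its slot, or creates one, then copies its values into instance variables.
; Each setter updates both the variable and the save object, then calls SaveData, which writes the slot immediately and prints success or error.
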(event `self.ReceiveInit`
  (bind _returnvalue (`GameplayStatics.DoesSaveGameExist` (`self.Slot Name`)))
  (if _returnvalue
    (bind _returnvalue_2 (`GameplayStatics.LoadGameFromSlot` (`self.Slot Name`)))
    (bind _assg_data_game (cast `/Game/Assets/Blueprints/GameMode/SG_DataGame` _returnvalue_2))
    (set `self.As SG Data Game` _assg_data_game)
    (else
      (bind _returnvalue_3 (`GameplayStatics.CreateSaveGameObject` "/Game/Assets/Blueprints/GameMode/SG_DataGame.SG_DataGame_C"))
      (set `self.As SG Data Game` _returnvalue_3)))
  (bind _as_sg_data_game (`self.As SG Data Game`)
    (:`then`
      (set `self.SensibilityMic` (`/Game/Assets/Blueprints/GameMode/SG_DataGame.SensibilityMic` _as_sg_data_game))
      (set `self.SensibilityMouse` (`/Game/Assets/Blueprints/GameMode/SG_DataGame.SensibilityMouse` _as_sg_data_game))
      (set `self.MethodDGI` (`/Game/Assets/Blueprints/GameMode/SG_DataGame.MethodDGI` _as_sg_data_game))
      (set `self.MethodRM` (`/Game/Assets/Blueprints/GameMode/SG_DataGame.MethodRM` _as_sg_data_game))
      (set `self.AudioMaster` (`/Game/Assets/Blueprints/GameMode/SG_DataGame.AudioMaster` _as_sg_data_game)))
    (:`else`)))

(event `SaveData`
  (bind _returnvalue (`GameplayStatics.SaveGameToSlot` (`self.As SG Data Game`) (`self.Slot Name`)))
  (`KismetSystemLibrary.PrintString` (select `bool` _returnvalue :`false` "SAVE ERROR" :`true` "SAVE GAME ") true true (struct :`R` 1.0 :`B` 0.0348 :`A` 1.0) 5.0))

(fn `SetAudioMaster`
  (params (AudioMaster :type "Float (double-precision)"))
  (bind _output_get (set `self.AudioMaster` AudioMaster))
  (bind _as_sg_data_game (`self.As SG Data Game`)
    (:`then`
      (set `/Game/Assets/Blueprints/GameMode/SG_DataGame.AudioMaster` _output_get _as_sg_data_game)
      (`self.SaveData`))
    (:`else`)))

(fn `SetMethodDGI`
  (params (MethodDGI :type "EDynamicGlobalIlluminationMethod Enum" :default "None"))
  (bind _output_get (set `self.MethodDGI` MethodDGI))
  (bind _as_sg_data_game (`self.As SG Data Game`)
    (:`then`
      (set `/Game/Assets/Blueprints/GameMode/SG_DataGame.MethodDGI` _output_get _as_sg_data_game)
      (`self.SaveData`))
    (:`else`)))

(fn `SetMethodRM`
  (params (MethodRM :type "EReflectionMethod Enum" :default "None"))
  (bind _output_get (set `self.MethodRM` MethodRM))
  (bind _as_sg_data_game (`self.As SG Data Game`)
    (:`then`
      (set `/Game/Assets/Blueprints/GameMode/SG_DataGame.MethodRM` _output_get _as_sg_data_game)
      (`self.SaveData`))
    (:`else`)))

(fn `SetSensibilityMic`
  (params (SensibilityMic :type "Float (double-precision)"))
  (bind _output_get (set `self.SensibilityMic` SensibilityMic))
  (bind _as_sg_data_game (`self.As SG Data Game`)
    (:`then`
      (set `/Game/Assets/Blueprints/GameMode/SG_DataGame.SensibilityMic` _output_get _as_sg_data_game)
      (`self.SaveData`))
    (:`else`)))

(fn `SetSensibilityMouse`
  (params (SensibilityMouse :type "Vector2D Structure"))
  (bind _output_get (set `self.SensibilityMouse` SensibilityMouse))
  (bind _as_sg_data_game (`self.As SG Data Game`)
    (:`then`
      (set `/Game/Assets/Blueprints/GameMode/SG_DataGame.SensibilityMouse` _output_get _as_sg_data_game)
      (`self.SaveData`))
    (:`else`)))