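; Master pickup actor that lets the player collect batteries, or matches, for the flashlight character.
; An overlap trigger stores the local player character and enables input only while that player is inside.
; Pressing Interact fires MulticastPickUpBattery, which increments the character's counter using this pickup's battery type and match amount.
; The actor is then destroyed through an RPC on BP_LightPlayerController so it disappears for server and clients.
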(event `self.OverlapTrigger.OnComponentBeginOverlap`
  (params (OverlappedComponent :type "PrimitiveComponent Object Reference") (OtherActor :type "Actor Object Reference") (OtherComp :type "PrimitiveComponent Object Reference") (OtherBodyIndex :type Integer) (bFromSweep :type Boolean) (SweepResult :type "HitResult Structure (by ref)"))
  ;[1 1 1] On Begin and end overlap we set the overlapped player variable if it's the player character
  (if (== OtherActor (`GameplayStatics.GetPlayerCharacter` 0))
    (set `self.OverlappedPlayer` OtherActor)
    (`self.EnableInput` (`GameplayStatics.GetPlayerController` 0))))

(event `self.OverlapTrigger.OnComponentEndOverlap`
  (params (OverlappedComponent :type "PrimitiveComponent Object Reference") (OtherActor :type "Actor Object Reference") (OtherComp :type "PrimitiveComponent Object Reference") (OtherBodyIndex :type Integer))
  ;[1 1 1] On Begin and end overlap we set the overlapped player variable if it's the player character
  (if (== (`GameplayStatics.GetPlayerCharacter` 0) OtherActor)
    (set `self.OverlappedPlayer` OtherActor)
    (`self.DisableInput` (`GameplayStatics.GetPlayerController` 0))))

(event `InputAction|Interact`
  (params (Key :type "Key Structure"))
  ;[1 1 1] Interact IA
  ;;[0 0.3259 0.5] On 'E' Button press, run the pick up code,
  (:`Pressed`
    (`self.Multicast PickUpBattery`)
    ;;[0 0.3259 0.5] Then Destroy the actor, for clients and server too.
    (bind _asbp_light_player_controller (cast `/Game/Market/AdvancedLightActors/Blueprints/Controller/BP_LightPlayerController` (`GameplayStatics.GetPlayerController` 0)))
    (`/Game/Market/AdvancedLightActors/Blueprints/Controller/BP_LightPlayerController.RPC Destroy Actor` _asbp_light_player_controller self)))

(event `Multicast PickUpBattery`
  ;[1 1 1] Increment the player's BatteryCounter, depending on which battery type this actor is.
  (bind _asbp_example_flashlight_character (cast `/Game/Market/AdvancedLightActors/Blueprints/CharacterBP/BP_ExampleFlashlightCharacter` (`self.OverlappedPlayer`)))
  (`/Game/Market/AdvancedLightActors/Blueprints/CharacterBP/BP_ExampleFlashlightCharacter.Increment Battery Counter` _asbp_example_flashlight_character (`self.BatteryType`) (`self.MatchesToAdd`)))

(fn `UserConstructionScript`)