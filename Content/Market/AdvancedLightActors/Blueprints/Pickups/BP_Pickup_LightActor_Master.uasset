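; Master pickup Blueprint that lets a player collect a light actor, carrying its saved battery power.
; Trigger overlap stores the overlapping actor and toggles Interact input on player controller 0.
; Unless a light is in use, Interact drops any carried one, then messages the player to spawn this pickup's light actor.
; The pickup is then destroyed through an RPC call on BP_LightPlayerController.
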(event `self.OverlapTrigger.OnComponentBeginOverlap`
  (params (OverlappedComponent :type "PrimitiveComponent Object Reference") (OtherActor :type "Actor Object Reference") (OtherComp :type "PrimitiveComponent Object Reference") (OtherBodyIndex :type Integer) (bFromSweep :type Boolean) (SweepResult :type "HitResult Structure (by ref)"))
  ;[1 1 1] On Begin and end overlap we set the overlapped player variable and enable the input of this actor.
  (set `self.OverlappedPlayer` OtherActor)
  (`self.EnableInput` (`GameplayStatics.GetPlayerController` 0)))

(event `self.OverlapTrigger.OnComponentEndOverlap`
  (params (OverlappedComponent :type "PrimitiveComponent Object Reference") (OtherActor :type "Actor Object Reference") (OtherComp :type "PrimitiveComponent Object Reference") (OtherBodyIndex :type Integer))
  ;[1 1 1] On Begin and end overlap we set the overlapped player variable and enable the input of this actor.
  (set `self.OverlappedPlayer` null)
  (`self.DisableInput` (`GameplayStatics.GetPlayerController` 0)))

(event `Save Battery Power`
  (params (SavedBatteryPower :type "Float (double-precision)"))
  ;[1 1 1] Sync Battery Power
  (set `self.SavedBatteryPower` SavedBatteryPower))

(event `InputAction|Interact`
  (params (Key :type "Key Structure"))
  ;[1 1 1] Event Interact - Pick Up LightActor / Drop Current one
  ;;[0 0.3259 0.5] On Interact Button Press - Check if the player is using a lightActor currently. only continue if not. Then check if he has a valid lightactor at all. (He's not using one, doesn't mean he doesn't have one.)
  (:`Pressed`
    (bind (_usinglightactor_ _lightactorref) (message `/Game/Market/AdvancedLightActors/Blueprints/Interfaces/BPI_LightActors.GetIsUsingLightActor?` (`self.OverlappedPlayer`)))
    (if (not _usinglightactor_)
      (`/Engine/EditorBlueprintResources/StandardMacros.IsValid` _lightactorref
        (:`Is Valid`
          ;;[0 0.3259 0.5] If he has one, drop it, and pick up a new one.
          (message `/Game/Market/AdvancedLightActors/Blueprints/Interfaces/BPI_LightActors.DropCurrentLightActor` (`self.OverlappedPlayer`) _lightactorref)
          (`self.Multicast PickupLightActor`))
        (:`Is Not Valid`
          ;;[0 0.3259 0.5] If he doesn't have one, just pick this one up.
          (`self.Multicast PickupLightActor`))))))

(event `Multicast PickupLightActor`
  ;[1 1 1] Pick Up LightActor - spawn lightActor in holster
  (message `/Game/Market/AdvancedLightActors/Blueprints/Interfaces/BPI_LightActors.SpawnPickedUpLightActor` (`self.OverlappedPlayer`) (`self.ActorToSpawn`) (`self.SavedBatteryPower`))
  (bind _asbp_light_player_controller (cast `/Game/Market/AdvancedLightActors/Blueprints/Controller/BP_LightPlayerController` (`GameplayStatics.GetPlayerController` 0)))
  (`/Game/Market/AdvancedLightActors/Blueprints/Controller/BP_LightPlayerController.RPC Destroy Actor` _asbp_light_player_controller self))

(fn `UserConstructionScript`)