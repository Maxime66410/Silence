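; Base actor for handheld light actors such as flashlights, with replicated toggle, three-level intensity cycling, sounds and hand-specific toggle montages.
; Server events relay to multicasts, while Tick updates the HUD power bar and drains battery at the current level's rate until the light dies.
; A forward sphere trace flickers the light on "LightFlicker"-tagged actors.
; BlindingSphereTrace increments blindness on head-bone hits through an interface, alongside adjustable cone angles for aiming.
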(event `self.ReceiveBeginPlay`
  (bind _hudreference (`self.HUDReference`))
  (bind _lightactorlight (`self.LightActorLight`))
  ;[1 1 1] Event Beginplay
  ;;[0 0.3259 0.5] Setting the default active light component(Still need to be set on each child actor!)
  (set `self.ActiveLightComponent` (`self.LightActorLight`))
  ;;[0 0.3259 0.5] Setting the default drain rate.
  (set `self.CurrentDrainRate` (`self.Level1DrainRate`))
  ;;[0 0.3259 0.5] Then show the power bar on the hud.
  (`KismetSystemLibrary.Delay` 0.5)
  (`/Engine/EditorBlueprintResources/StandardMacros.IsValid` _hudreference
    (:`Is Valid`
      (`/Game/Market/AdvancedLightActors/Widgets/W_PlayerHUD.Show Battery Power Bar` _hudreference)
      ;;[0 0.3259 0.5] Then set the default cone angles of the light. (Used for the Blinding system of the flashlight.) The system reverts the values of the cone angles to this value when the player stops aiming with the flashlight.
      (set `self.DefaultOuterConeAngle` (`SpotLightComponent.OuterConeAngle` _lightactorlight))
      (set `self.DefaultInnerConeAngle` (`SpotLightComponent.InnerConeAngle` _lightactorlight)))))

(event `Multicast Flicker Light`
  ;[1 1 1] Multicast Light Flickering Events
  ;;[0 0.3259 0.5] Multicast Flicker Light
  (set `self.IsFlickering?` true)
  (`LightComponent.SetIntensity` (`self.ActiveLightComponent`) (`KismetMathLibrary.RandomFloatInRange` 0.0 (`self.CurrentIntensity`))))

(event `/Game/Market/AdvancedLightActors/Blueprints/Interfaces/BPI_LightActors.Holstered`
  ;[1 1 1] Interface Events
  ;;[0 0.3259 0.5] Event Holstered - "isPlayerUsingLightActor?" is used when the system needs to check if the light actor is equipped ( but without using a reference to the player.. used in BP_Camera_Master for example.)
  (set `self.IsPlayerUsingLightActor?` false)
  (if (`self.ShouldHideOnHolstered?`)
    (`self.SetActorHiddenInGame` true)))

(event `Multicast Switch Intensity UP`
  ;[1 1 1] Intensity Switching Logic
  ;;[0 0.3259 0.5] Switch Intensity Up
  (`self.FlashlightNotOut?`
    (:`true`
      (switch `int` (`self.IntensityIndex`)
        (:`0`
          (set `self.IntensityIndex` 1)
          (set `self.CurrentIntensity` (`self.Level2Intensity`))
          (set `self.CurrentDrainRate` (`self.Level2DrainRate`)))
        (:`1`
          (set `self.IntensityIndex` 2)
          (set `self.CurrentIntensity` (`self.Level3Intensity`))
          (set `self.CurrentDrainRate` (`self.Level3DrainRate`)))
        (:`2`
          (set `self.IntensityIndex` 0)
          (set `self.CurrentIntensity` (`self.Level1Intensity`))
          (set `self.CurrentDrainRate` (`self.Level1DrainRate`))))
      (`LightComponent.SetIntensity` (`self.ActiveLightComponent`) (`self.CurrentIntensity`)))))

(event `Multicast Toggle Active Light`
  (bind _level1intensity (`self.Level1Intensity`))
  (bind _activelightcomponent (`self.ActiveLightComponent`))
  (bind (_lightactorholstersocket _lightactorrighthandsocket _lightactorlefthandsocket _pickupactorclass _shouldusetogglemontage_ _lightactorrighthandtogglemontage _lightactorlefthandtogglemontage _togglesound) (break `/Game/Market/AdvancedLightActors/Blueprints/Struct_LightActorInfo` (`self.LightActorInfo`)))
  ;[1 1 1] Toggling The Active Light Component On/Off
  ;;[0 0.3259 0.5] Multicast Toggle Flashlight
  (if (not _shouldusetogglemontage_)
    ;;;[0 0.3259 0.5] If no toggle animation - play sound instantly
    (`GameplayStatics.PlaySoundAtLocation` _togglesound (`self.K2_GetActorLocation`) (struct) 1.0 1.0 0.0 null null null null))
  (if (`self.IsTurnedOn?`)
    (set `self.IsTurnedOn?` false)
    (`LightComponent.SetIntensity` _activelightcomponent 0.0)
    (set `self.CurrentIntensity` 0.0)
    (`self.TurnedOff`)
    (else
      (set `self.IsTurnedOn?` true)
      (`LightComponent.SetIntensity` _activelightcomponent _level1intensity)
      (set `self.CurrentIntensity` _level1intensity)
      (`self.TurnedOn`))))

(event `/Game/Market/AdvancedLightActors/Blueprints/Interfaces/BPI_LightActors.Equipped`
  ;[1 1 1] Interface Events
  ;;[0 0.3259 0.5] Event Equipped
  (set `self.IsPlayerUsingLightActor?` true)
  (if (`self.ShouldHideOnHolstered?`)
    (`self.SetActorHiddenInGame` false)))

(event `Server Switch Intensity UP`
  ;[1 1 1] Intensity Switching Logic
  ;;[0 0.3259 0.5] Switch Intensity Up
  ;;;[0 0.3259 0.5] Server Switch intensity up
  (`self.Multicast Switch Intensity UP`))

(event `Multicast Stop Flickering`
  ;[1 1 1] Multicast Light Flickering Events
  ;;[0 0.3259 0.5] Multicast Stop Flickering
  (set `self.IsFlickering?` false)
  (`LightComponent.SetIntensity` (`self.ActiveLightComponent`) (`self.CurrentIntensity`)))

(event `self.ReceiveTick`
  (params (DeltaSeconds :type "Float (single-precision)"))
  (bind _hudreference (`self.HUDReference`))
  (bind _batterypower (`self.BatteryPower`))
  ;[1 1 1] Event Tick
  (`|ExecutionSequence`
    (:`then_0`
      ;;[0 0.3259 0.5] Updating the power bar's percentage on every tick.
      (`/Engine/EditorBlueprintResources/StandardMacros.IsValid` _hudreference
        (:`Is Valid`
          (`/Game/Market/AdvancedLightActors/Widgets/W_PlayerHUD.Update Battery Power Bar` _hudreference (/ (`self.BatteryPower`) 100.0)))))
    (:`then_1`
      ;;[0 0.3259 0.5] Battery Power Draining Logic
      (if (`self.NeedsBatteries?`)
        ;;;[0 0.3259 0.5] If turned on, wait "X" seconds, then decrement 1 from the battery power.
        (if (`self.IsTurnedOn?`)
          (`KismetSystemLibrary.Delay` (`self.CurrentDrainRate`))
          (set `self.BatteryPower` (`KismetMathLibrary.FClamp` (- _batterypower 1.0) 0.0 100.0))
          ;;;[0 0.3259 0.5] Then if the battery power is 0, the light actor is out, and toggle the active light component ( turn it off)
          (if (<= _batterypower 0.0)
            (`/Engine/EditorBlueprintResources/StandardMacros.DoOnce` false :!label _label
              (:`Completed`
                (`self.Server LightActor Out`)
                (`self.Server Toggle Active Light`))))
          (else
            (goto _label :!via `Reset`)))))
    (:`then_2`
      ;;[0 0.3259 0.5] If The LightActor Is turned on, do a LightFlicker Trace in each .1 second
      (if (and (`self.IsTurnedOn?`) (`self.ShouldUseLightFlickering?`))
        (`KismetSystemLibrary.Delay` 0.1)
        (`self.LightFlickerSphereTrace`)))))

(event `/Game/Market/AdvancedLightActors/Blueprints/Interfaces/BPI_LightActors.TurnedOn`
  ;[1 1 1] Interface Events
  ;;[0 0.3259 0.5] Event Turned On - If you want to add something extra (like a particle system for all child actors in common, add it here.)
)

(event `Server Toggle Active Light`
  ;[1 1 1] Toggling The Active Light Component On/Off
  ;;[0 0.3259 0.5] Server Toggle Active Light
  (`self.Multicast Toggle Active Light`))

(event `Multicast Switch Intensity DOWN`
  ;[1 1 1] Intensity Switching Logic
  ;;[0 0.3259 0.5] Switch Intensity Down
  (`self.FlashlightNotOut?`
    (:`true`
      (switch `int` (`self.IntensityIndex`)
        (:`0`
          (set `self.IntensityIndex` 2)
          (set `self.CurrentIntensity` (`self.Level3Intensity`))
          (set `self.CurrentDrainRate` (`self.Level3DrainRate`)))
        (:`1`
          (set `self.IntensityIndex` 0)
          (set `self.CurrentIntensity` (`self.Level1Intensity`))
          (set `self.CurrentDrainRate` (`self.Level1DrainRate`)))
        (:`2`
          (set `self.IntensityIndex` 1)
          (set `self.CurrentIntensity` (`self.Level2Intensity`))
          (set `self.CurrentDrainRate` (`self.Level2DrainRate`))))
      (`LightComponent.SetIntensity` (`self.ActiveLightComponent`) (`self.CurrentIntensity`)))))

(event `Multicast Play LightActor Sound`
  (params (Sound :type "SoundBase Object Reference"))
  ;[1 1 1] Toggling The Active Light Component On/Off
  ;;[0 0.3259 0.5] Play LightActor Sound - Child Related - play any replicated selected sound. (used in camera master BP)
  (`GameplayStatics.PlaySoundAtLocation` Sound (`self.K2_GetActorLocation`) (struct) 1.0 1.0 0.0 null null null null))

(event `Sync Battery Power`
  (params (BatteryPower :type "Float (double-precision)"))
  ;[1 1 1] Event Sync Battery Power (Used in Character BP,  at "SpawnLightActorAtHolster")
  (set `self.BatteryPower` BatteryPower))

(event `/Game/Market/AdvancedLightActors/Blueprints/Interfaces/BPI_LightActors.TurnedOff`
  ;[1 1 1] Interface Events
  ;;[0 0.3259 0.5] Then deactivate it here.
)

(event `MulticastLightActorOut`
  ;[1 1 1] Event Tick
  ;;[0 0.3259 0.5] Multicast Light Actor Out
  (set `self.IsLightActorOut?` true))

(event `Multicast Play Toggle Sound`
  ;[1 1 1] Toggling The Active Light Component On/Off
  ;;[0 0.3259 0.5] Play Toggle Sound - gets called from AnimNotify
  (`GameplayStatics.PlaySoundAtLocation` (`.ToggleSound_28_214974CE45721FD04E6B84901D197729` (break `/Game/Market/AdvancedLightActors/Blueprints/Struct_LightActorInfo` (`self.LightActorInfo`))) (`self.K2_GetActorLocation`) (struct) 1.0 1.0 0.0 null null null null))

(event `Server Switch intensity down`
  ;[1 1 1] Intensity Switching Logic
  ;;[0 0.3259 0.5] Switch Intensity Down
  ;;;[0 0.3259 0.5] Server Switch Intensity down
  (`self.Multicast Switch Intensity DOWN`))

(event `Server Play LightActor Sound`
  (params (Sound :type "SoundBase Object Reference"))
  ;[1 1 1] Toggling The Active Light Component On/Off
  ;;[0 0.3259 0.5] Play LightActor Sound - Child Related - play any replicated selected sound. (used in camera master BP)
  (`self.Multicast Play LightActor Sound` Sound))

(event `Server LightActor Out`
  ;[1 1 1] Event Tick
  ;;[0 0.3259 0.5] Server LightActor Out
  (`self.MulticastLightActorOut`))

(event `/Game/Market/AdvancedLightActors/Blueprints/Interfaces/BPI_LightActors.ToggleDebugging`
  (params (`DebuggingOn?` :type Boolean))
  (bind _arrow (`self.Arrow`))
  ;[1 1 1] Interface Events
  ;;[0 0.3259 0.5] Event Toggle Debugging - Show hidden components. If you want you can overwrite this event, or print out any variables or anything when debugging is on. It helps you a lot to find out what is causing a problem.
  (if `DebuggingOn?`
    (`SceneComponent.SetHiddenInGame` _arrow false false)
    (else
      (`SceneComponent.SetHiddenInGame` _arrow true false))))

(event `Server Play Toggle Sound`
  ;[1 1 1] Toggling The Active Light Component On/Off
  ;;[0 0.3259 0.5] Play Toggle Sound - gets called from AnimNotify
  (`self.Multicast Play Toggle Sound`))

(event `Server Restore Power`
  ;[1 1 1] Event Tick
  ;;[0 0.3259 0.5] Server Restore Power
  (`self.Multicast Restore Power`))

(event `Multicast Restore Power`
  ;[1 1 1] Event Tick
  ;;[0 0.3259 0.5] Multicast Restore Power
  (set `self.IsLightActorOut?` false)
  (set `self.BatteryPower` 100.0))

(event `/Game/Market/AdvancedLightActors/Blueprints/Interfaces/BPI_LightActors.OuterConeAngleChanged`
  (params (`New Amount` :type "Float (double-precision)"))
  ;[1 1 1] Interface Events
  ;;[0 0.3259 0.5] Set Outer and Inner Cone Angle - called from the character BP, when the palyer starts aiming with a flashlight. It's related only for flashlight actros currently.
  (`SpotLightComponent.SetOuterConeAngle` (`self.LightActorLight`) `New Amount`))

(event `Multicast Play Toggle Anim Montage`
  (params (Character :type "Character Object Reference") (`IsLeftHanded?` :type Boolean))
  (bind (_lightactorholstersocket _lightactorrighthandsocket _lightactorlefthandsocket _pickupactorclass _shouldusetogglemontage_ _lightactorrighthandtogglemontage _lightactorlefthandtogglemontage) (break `/Game/Market/AdvancedLightActors/Blueprints/Struct_LightActorInfo` (`self.LightActorInfo`)))
  ;[1 1 1] Toggling The Active Light Component On/Off
  ;;[0 0.3259 0.5] Multicast Toggle Light Anim depending on preferred hand. The anim montage has to be set up in the LightActorInfo structure variable
  (`/Engine/EditorBlueprintResources/StandardMacros.IsValid` Character
    (:`Is Valid`
      (if (not `IsLeftHanded?`)
        (`Character.PlayAnimMontage` Character _lightactorrighthandtogglemontage 1.0 "None")
        (else
          (`Character.PlayAnimMontage` Character _lightactorlefthandtogglemontage 1.0 "None"))))))

(event `/Game/Market/AdvancedLightActors/Blueprints/Interfaces/BPI_LightActors.InnerConeAngleChanged`
  (params (`New Amount` :type "Float (double-precision)"))
  ;[1 1 1] Interface Events
  ;;[0 0.3259 0.5] Set Outer and Inner Cone Angle - called from the character BP, when the palyer starts aiming with a flashlight. It's related only for flashlight actros currently.
  (`SpotLightComponent.SetInnerConeAngle` (`self.LightActorLight`) `New Amount`))

(fn `BlindingSphereTrace`
  (bind _arrow (`self.Arrow`))
  (bind _returnvalue (`SceneComponent.K2_GetComponentLocation` _arrow))
  ;[1 1 1] Blinding Sphere Trace- used in Flashlight T1 and T2 when aiming with flashlight
  ;;[0 0.3259 0.5] Same Locations and checks as light flickering
  (bind _debuggingon_ (message `/Game/Market/AdvancedLightActors/Blueprints/Interfaces/BPI_DeveloperOptions.GetIsDebuggingOn?` (`self.GetOwner`)))
  (bind (_outhit _returnvalue_2) (`KismetSystemLibrary.SphereTraceSingle` _returnvalue (+ _returnvalue (* (`SceneComponent.GetForwardVector` _arrow) (`self.FlickerTraceDistance`))) 10.0 "TraceTypeQuery1" false (`|MakeArray` (`self.GetOwner`) self :!type "Actor Object Reference") (select `bool` _debuggingon_ :`true` "ForDuration" :!type "EDrawDebugTrace Enum") true (struct :`R` 0.5 :`B` 0.002984 :`A` 1.0)))
  ;;[0 0.3259 0.5] Check if the actor has the BPI_LightActors interface in it, and check if the trace hits the head bone of the actor. (send a message to the actor the trace hits.) this message needs to be written in each actor. it needs to return the head bone of the mesh. (check it in the skeleton, then write it in.)
  (if _returnvalue_2
    (bind (_bblockinghit _binitialoverlap _time _distance _location _impactpoint _normal _impactnormal _physmat _hitactor _hitcomponent _hitbonename) (`GameplayStatics.BreakHitResult` _outhit))
    (if (`KismetSystemLibrary.DoesImplementInterface` _hitactor "/Game/Market/AdvancedLightActors/Blueprints/Interfaces/BPI_FlashlightBlinding.BPI_FlashlightBlinding_C")
      (bind _headbonename (message `/Game/Market/AdvancedLightActors/Blueprints/Interfaces/BPI_FlashlightBlinding.GetHeadBone` _hitactor))
      (if (== _headbonename _hitbonename)
        ;;[0 0.3259 0.5] Then increment the blindness value of the actor. (event needs to be written in the actor)
        (message `/Game/Market/AdvancedLightActors/Blueprints/Interfaces/BPI_FlashlightBlinding.IncrementBlindedValue` _hitactor (`self.BlindAmountToAdd`))))))

(fn `GetBatteries`
  (returns (`Battery Amount` :type Integer))
  (return 0))

(fn `GetIsUsingLightActor?`
  (returns (`UsingLightActor?` :type Boolean) (LightActorRef :type "/Game/Market/AdvancedLightActors/Blueprints/LightActors/BP_LightActor_Master Object Reference"))
  (return false null))

(fn `GetLightActorOwnerPawn`
  (returns (`Player Pawn` :type "Pawn Object Reference"))
  (return null))

(fn `LightFlickerSphereTrace`
  (bind _arrow (`self.Arrow`))
  (bind _returnvalue (`SceneComponent.K2_GetComponentLocation` _arrow))
  ;[1 1 1] Light Flicker Sphere Trace
  ;;[0 0.3259 0.5] On every tick, do a sphere trace from the arrow's location, in forward direction for the X amount that's set in the FlickerTraceDistance variable.
  ;;;[0 0.3259 0.5] This gets the owner's (player) "DebuggingOn" bool, without the need to use a  reference
  (bind _debuggingon_ (message `/Game/Market/AdvancedLightActors/Blueprints/Interfaces/BPI_DeveloperOptions.GetIsDebuggingOn?` (`self.GetOwner`)))
  (bind (_outhit _returnvalue_2) (`KismetSystemLibrary.SphereTraceSingle` _returnvalue (+ _returnvalue (* (`SceneComponent.GetForwardVector` _arrow) (`self.FlickerTraceDistance`))) 15.0 "TraceTypeQuery1" false (`|MakeArray` (`self.GetOwner`)) (select `bool` _debuggingon_ :`true` "ForDuration" :!type "EDrawDebugTrace Enum") true (struct :`G` 0.325934 :`B` 0.5 :`A` 1.0)))
  ;;[0 0.3259 0.5] If the line trace overlaps with an actor that has 'LightFlicker' TAG attached to it, it runs the Flicker Light code.
  (if _returnvalue_2
    (bind (_bblockinghit _binitialoverlap _time _distance _location _impactpoint _normal _impactnormal _physmat _hitactor) (`GameplayStatics.BreakHitResult` _outhit))
    (`/Engine/EditorBlueprintResources/StandardMacros.IsValid` _hitactor
      (:`Is Valid`
        (if (`self.ActorHasTag` _hitactor "LightFlicker")
          (`self.Multicast Flicker Light`)
          (else
            ;;;[1 0 0] If the light is already flickering, and the trace stops overlapping with something, or overlaps an actor what doesn't have the tag attached to it, it stops flickering.
            (if (`self.IsFlickering?`) :!label _label
              (`self.Multicast Stop Flickering`))))))
    (else
      (goto _label))))

(fn `UserConstructionScript`)