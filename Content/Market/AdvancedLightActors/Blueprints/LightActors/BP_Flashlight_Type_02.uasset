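; BP_Flashlight_Type_02 is a flashlight light-actor variant that extends parent tick and construction logic with source-light switching and a blinding trace.
; On tick it calls the parent, passes through a 0.1-second Delay, then asks its owner whether the flashlight is being aimed and, if so, runs BlindingSphereTrace.
; The turned-on event sets SourceLight to half of Level1Intensity, and the turned-off event sets it to zero.
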(event `self.ReceiveTick`
  (params (DeltaSeconds :type "Float (single-precision)"))
  ;[1 1 1] Event Tick - if player is aiming, do a blindingSphereTrace
  (`parent.ReceiveTick` DeltaSeconds)
  (`KismetSystemLibrary.Delay` 0.1)
  (bind _isaimingflashlight_ (message `/Game/Market/AdvancedLightActors/Blueprints/Interfaces/BPI_FlashlightBlinding.GetIsAimingFlashlight?` (`self.GetOwner`)))
  (if _isaimingflashlight_
    (`self.BlindingSphereTrace`)))

(event `/Game/Market/AdvancedLightActors/Blueprints/Interfaces/BPI_LightActors.TurnedOn`
  ;[1 1 1] On Turned On / Off , toggle switching on / off the source light
  (`LightComponent.SetIntensity` (`self.SourceLight`) (/ (`self.Level1Intensity`) 2.0)))

(event `/Game/Market/AdvancedLightActors/Blueprints/Interfaces/BPI_LightActors.TurnedOff`
  ;[1 1 1] On Turned On / Off , toggle switching on / off the source light
  (`LightComponent.SetIntensity` (`self.SourceLight`) 0.0))

(fn `UserConstructionScript`
  (`parent.UserConstructionScript`))