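; Master Blueprint for lantern light actors, extending a parent light actor with a point light, a fire particle effect and physics-based swinging.
; BeginPlay sets the lantern's point light as the active light component.
; Equipped and Holstered events unlock or lock the physics constraint's Swing2 angular limit, so the lantern swings only while equipped.
; Turn on and off events toggle the fire particle through a server-to-multicast event pair for replication.
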(event `EnableConstraintMotion`
  ;[1 1 1] Enabling / Disabling swinging.
  (`PhysicsConstraintComponent.SetAngularSwing2Limit` (`self.LanternPhysicsConstraint`) "ACM_Limited" 35.0))

(event `self.ReceiveBeginPlay`
  ;[1 1 1] Beginplay - set active light component
  (`parent.ReceiveBeginPlay`)
  (set `self.ActiveLightComponent` (`self.LanternPointLight`)))

(event `/Game/Market/AdvancedLightActors/Blueprints/Interfaces/BPI_LightActors.TurnedOn`
  ;[1 1 1] Turning On / Off Fire Particle
  (`self.Server Toggle Active Particle System` true))

(event `/Game/Market/AdvancedLightActors/Blueprints/Interfaces/BPI_LightActors.Holstered`
  ;[1 1 1] Interface Events
  ;;[0 0.3259 0.5] Event Holstered - Disabling the back and forth swinging of mesh.
  (`parent.Holstered`)
  (`self.DisableConstraintMotion`))

(event `DisableConstraintMotion`
  ;[1 1 1] Enabling / Disabling swinging.
  (`PhysicsConstraintComponent.SetAngularSwing2Limit` (`self.LanternPhysicsConstraint`) "ACM_Locked" 0.0))

(event `/Game/Market/AdvancedLightActors/Blueprints/Interfaces/BPI_LightActors.TurnedOff`
  ;[1 1 1] Turning On / Off Fire Particle
  (`self.Server Toggle Active Particle System` false))

(event `/Game/Market/AdvancedLightActors/Blueprints/Interfaces/BPI_LightActors.Equipped`
  ;[1 1 1] Interface Events
  ;;[0 0.3259 0.5] Event Equipped - Enabling the swing motion.
  (`parent.Equipped`)
  (`self.EnableConstraintMotion`))

(event `Server Toggle Active Particle System`
  (params (`On?` :type Boolean))
  ;[1 1 1] Replicated Particle System Toggling
  (`self.Multicast Toggle Active Particle System` `On?`))

(event `Multicast Toggle Active Particle System`
  (params (`On?` :type Boolean))
  (bind _pstorchfire (`self.PSTorchFire`))
  ;[1 1 1] Replicated Particle System Toggling
  (if `On?`
    (`ActorComponent.Activate` _pstorchfire false)
    (else
      (`ActorComponent.Deactivate` _pstorchfire))))

(fn `UserConstructionScript`
  (`parent.UserConstructionScript`))