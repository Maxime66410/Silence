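; Handheld camera light actor with flashlight, night vision, zoom, recording and photo taking, extending the light actor parent's logic.
; A scene capture feeds a render target on the screen widget; fullscreen aiming switches to the camera's viewpoint.
; While recording, per-tick traces find BPI_CameraInteraction actors, triggering interactions or enabling photos, optionally requiring a specific component.
; Battery drains via a Tick delay that active features shorten; depletion resets the camera.
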(event `self.ReceiveTick`
  (params (DeltaSeconds :type "Float (single-precision)"))
  (bind _hudreference (`self.HUDReference`))
  (bind _batterypower (`self.BatteryPower`))
  ;[1 1 1] Event Tick
  (`|ExecutionSequence`
    (:`then_0`
      ;;[0 0.3259 0.5] On every tick, if the HUD is valid (isn't fullscreen aiming) update the HUD's power bar.
      (`/Engine/EditorBlueprintResources/StandardMacros.IsValid` _hudreference
        (:`Is Valid`
          (`/Game/Market/AdvancedLightActors/Widgets/W_PlayerHUD.Update Battery Power Bar` _hudreference (/ (`self.BatteryPower`) 100.0)))))
    (:`then_1`
      ;;[0 0.3259 0.5] Update the screen widget's power bar on every tick too.
      (`/Game/Market/AdvancedLightActors/Widgets/W_BatteryBar.Update Battery Power Bar` (`/Game/Market/AdvancedLightActors/Widgets/W_CameraScreen.W_BatteryBar` (`self.CameraWidgetRef`)) (/ (`self.BatteryPower`) 100.0)))
    (:`then_2`
      ;;[0 0.3259 0.5] If the camera is recording, and found a target, but searching for the required component, call the "CameraPhotoLineTrace" if the camera is recording but doesn't found the target, call the "InteractionLineTrace"
      (if (`self.IsRecording?`)
        (if (`self.PhotoTargetFound?`)
          (if (`self.SearchingForComponent?`)
            (`self.CameraPhotoLineTrace`)
            (else
              (`self.InteractionLineTrace`)))
          (else
            (`self.InteractionLineTrace`)))))
    (:`then_3`
      ;;[0 0.3259 0.5] On every tick, if the player is using the camera, wait the "DrainRate's amount" then decrement it's battery power by 1,  and if the power is 0 , the camera is out.
      (if (`self.IsPlayerUsingLightActor?`)
        (`KismetSystemLibrary.Delay` (`self.CurrentDrainRate`))
        (set `self.BatteryPower` (`KismetMathLibrary.FClamp` (- _batterypower 1.0) 0.0 100.0))
        (if (<= _batterypower 0.0)
          (`/Engine/EditorBlueprintResources/StandardMacros.DoOnce` false :!label _label
            (:`Completed`
              (`self.Server LightActor Out`)))
          (else
            (goto _label :!via `Reset`)))))
    (:`then_4`
      ;;[0 0.3259 0.5] If The LightActor Is turned on, do a LightFlicker Trace in each .1 second
      (if (and (`self.IsTurnedOn?`) (`self.ShouldUseLightFlickering?`))
        (`KismetSystemLibrary.Delay` 0.1)
        (`self.LightFlickerSphereTrace`)))))

(event `self.ReceiveBeginPlay`
  ;[1 1 1] Event Beginplay
  ;;[0 0.3259 0.5] Call the parent's beginplay, then set the camera widget ref(so it can be used later) and check if the player is locally controlled.
  (`parent.ReceiveBeginPlay`)
  (bind _asw_camera_screen (cast `/Game/Market/AdvancedLightActors/Widgets/W_CameraScreen` (`WidgetComponent.GetUserWidgetObject` (`self.CameraWidget`))))
  (set `self.CameraWidgetRef` _asw_camera_screen)
  (bind _player_pawn (message `/Game/Market/AdvancedLightActors/Blueprints/Interfaces/BPI_LightActors.GetLightActorOwnerPawn` (`self.GetOwner`)))
  (if (`Pawn.IsLocallyControlled` _player_pawn)
    ;;[0 0.3259 0.5] Create a render target for locally controlled characters, and add it as the scene capture component's texture target,, so it records the screen to it, then add it as te camera widget's render target, so it's projected to the widget.
    (bind _returnvalue (`KismetRenderingLibrary.CreateRenderTarget2D` 1920 1080))
    (set `/Game/Market/AdvancedLightActors/Widgets/W_CameraScreen.RenderTarget` _returnvalue (`self.CameraWidgetRef`))
    (set `SceneCaptureComponent2D.TextureTarget` _returnvalue (`self.SceneCaptureComponent2D`))
    ;;[0 0.3259 0.5] Then sync the battery amount of the widget, and set the camera's default location, so it can be modified later, and returned back to the default location.
    (bind _battery_amount (message `/Game/Market/AdvancedLightActors/Blueprints/Interfaces/BPI_LightActors.GetBatteries` (`self.GetOwner`)))
    (`self.BatteryAmountChanged` _battery_amount)
    (set `self.DefaultCameraLocation` (`SceneComponent.RelativeLocation` (`self.Camera`)))))

(event `BatteryAmountChanged`
  (params (NewAmount :type Integer))
  ;[1 1 1] Battery Related Events
  ;;[0 0.3259 0.5] BatteryAmount Changed - set the widget's battery counter to the new value.
  (`TextBlock.SetText` (`/Game/Market/AdvancedLightActors/Widgets/W_CameraScreen.T_BatteryCounter` (`self.CameraWidgetRef`)) (`KismetTextLibrary.Conv_IntToText` NewAmount)))

(event `Start Recording`
  ;[1 1 1] Recording Events
  ;;[0 0.3259 0.5] Start Recording - update the recording text, then set the recording bools to true, and decrement the drain rate(make the battery drain down faster)
  (`self.Update Recording Text` "STOP" (struct :`R` 0.002465 :`G` 1.0 :`A` 1.0))
  (set `/Game/Market/AdvancedLightActors/Widgets/W_CameraScreen.IsRecording?` true (`self.CameraWidgetRef`))
  (set `self.IsRecording?` true)
  (`self.DecrementDrainRate` (`self.RecordingDrainRate`)))

(event `Start Fullscreen Aiming`
  (bind _camerawidgetref (`self.CameraWidgetRef`))
  ;[1 1 1] Fullscreen aiming logic ( called from CharacterBP)
  ;;[0 0.3259 0.5] Start Fullscreen aiming - we must hide the "BackgroundBorder" since in FS aiming the system uses the camera's viewpoint. - then, add the screen widget to the player's viewport - then set the camera's location in the place of the SCC2D component.
  (set `self.IsFullscreenAiming?` true)
  (`Widget.SetVisibility` (`/Game/Market/AdvancedLightActors/Widgets/W_CameraScreen.BackgroundBorder` _camerawidgetref) "Hidden")
  (`UserWidget.AddToViewport` _camerawidgetref 0)
  (`SceneComponent.K2_SetRelativeLocation` (`self.Camera`) (`SceneComponent.RelativeLocation` (`self.SceneCaptureArrow`)) false false)
  (`PlayerController.SetViewTargetWithBlend` (`GameplayStatics.GetPlayerController` 0) self 0.0 "VTBlend_Linear" 0.0 false)
  (`Widget.RemoveFromParent` (`self.HUDReference`)))

(event `PhotogenicTargetFound`
  (params (TargetActor :type "Actor Object Reference") (`NeedsSpecificComponent?` :type Boolean))
  (bind _i_camera_focus (`/Game/Market/AdvancedLightActors/Widgets/W_CameraScreen.I_Camera_Focus` (`self.CameraWidgetRef`)))
  ;[1 1 1] Photo Creation Events
  ;;[0 0.3259 0.5] If the "InteractionLineTrace" finds a target, set it as the target actor, set the required variables. - if the target actor needs a specific component to be photographed, set the "SearchingForComponent" bool to true, and the system starts the "CameraPhotoLineTrace" by every tick, searching for the required component.
  (set `self.PhotoTargetActor` TargetActor)
  (set `self.PhotoTargetFound?` true)
  (`Image.SetBrushFromTexture` (`/Game/Market/AdvancedLightActors/Widgets/W_CameraScreen.I_Camera_Focus` (`self.CameraWidgetRef`)) "/Game/Market/AdvancedLightActors/Widgets/Textures/T_Camera_Focus_Tight.T_Camera_Focus_Tight" true)
  (if `NeedsSpecificComponent?`
    (set `self.SearchingForComponent?` true)
    (`Image.SetColorAndOpacity` _i_camera_focus (struct :`R` 0.5 :`B` 0.002984 :`A` 1.0))
    (else
      (set `self.CanTakePhoto?` true)
      (`Image.SetColorAndOpacity` _i_camera_focus (struct :`R` 0.002465 :`G` 1.0 :`A` 1.0)))))

(event `StartNightVision`
  (bind _scenecapturecomponent2d (`self.SceneCaptureComponent2D`))
  ;[1 1 1] Toggle NightVision On / Off
  ;;[0 0.3259 0.5] Start Night Vision - decrement the drain rate, then if fullscreen, enable the night vision post process to the whole screen, and set the night vision icon visible. If not full screen, set the scene capture component's post process to the night vision settings, making only the screen of the camera use the night vision post process.
  (`self.DecrementDrainRate` (`self.NightVisionDrainRate`))
  (if (`self.IsFullscreenAiming?`)
    (set `PostProcessComponent.bEnabled` true (`self.NightVision`))
    (set `self.IsNightVisionOn?` true)
    (`Widget.SetVisibility` (`/Game/Market/AdvancedLightActors/Widgets/W_CameraScreen.I_NightVisionOn` (`self.CameraWidgetRef`)) "Visible")
    (else
      (set `SceneCaptureComponent2D.PostProcessSettings` (`self.NightVisionPPSettings`) _scenecapturecomponent2d)
      (set `SceneCaptureComponent2D.CaptureSource` "SCS_FinalColorLDR" _scenecapturecomponent2d)
      (set `self.IsNightVisionOn?` true)
      (`Widget.SetVisibility` (`/Game/Market/AdvancedLightActors/Widgets/W_CameraScreen.I_NightVisionOn` (`self.CameraWidgetRef`)) "Visible"))))

(event `CameraZoomIn`
  (params (ZoomAmount :type "Float (double-precision)"))
  (bind _pb_zoomlevel (`/Game/Market/AdvancedLightActors/Widgets/W_CameraScreen.PB_ZoomLevel` (`self.CameraWidgetRef`)))
  (bind _fovangle (`SceneCaptureComponent2D.FOVAngle` (`self.SceneCaptureComponent2D`)))
  (bind _pb_zoomlevel_2 (`/Game/Market/AdvancedLightActors/Widgets/W_CameraScreen.PB_ZoomLevel` (`self.CameraWidgetRef`)))
  (bind _fieldofview (`CameraComponent.FieldOfView` (`self.Camera`)))
  ;[1 1 1] Camera Zoom In / Out Functions - From CharacterBP
  ;;[0 0.3259 0.5] Camera Zoom In - if the FOV is greater than the min zoom FOV (maximum amount the player can zoom in) - decerase the FOV of the camera by ZoomAmount.
  (if (`self.IsFullscreenAiming?`)
    (if (> _fieldofview (`self.MinZoomFOV`))
      (`CameraComponent.SetFieldOfView` (`self.Camera`) (- _fieldofview ZoomAmount))
      (`ProgressBar.SetPercent` _pb_zoomlevel (+ (`ProgressBar.Percent` _pb_zoomlevel) 0.25)))
    (elif (> _fovangle (`self.MinZoomFOV`))
      (set `SceneCaptureComponent2D.FOVAngle` (- _fovangle ZoomAmount) (`self.SceneCaptureComponent2D`))
      (`ProgressBar.SetPercent` _pb_zoomlevel_2 (+ (`ProgressBar.Percent` _pb_zoomlevel_2) 0.25)))))

(event `DecrementDrainRate`
  (params (Amount :type "Float (double-precision)"))
  ;[1 1 1] Battery Related Events
  ;;[0 0.3259 0.5] Decerement Drain Rate - Make the battery drain down faster ( because on every tick, the delay node's amount is less, so it waits less amount of time to decrement the battery.)
  (set `self.CurrentDrainRate` (`KismetMathLibrary.FClamp` (- (`self.CurrentDrainRate`) Amount) 0.0 (`self.Level1DrainRate`))))

(event `StopRecording`
  ;[1 1 1] Recording Events
  ;;[0 0.3259 0.5] Stop Recording - Reset everything to default.
  (`self.Update Recording Text` "REC" (struct :`R` 0.5 :`B` 0.002984 :`A` 1.0))
  (set `/Game/Market/AdvancedLightActors/Widgets/W_CameraScreen.IsRecording?` false (`self.CameraWidgetRef`))
  (`/Game/Market/AdvancedLightActors/Widgets/W_CameraScreen.Clear Recording Time Passed` (`self.CameraWidgetRef`))
  (set `self.IsRecording?` false)
  (`self.IncrementDrainRate` (`self.RecordingDrainRate`))
  (`self.PhotogenicTargetLost`))

(event `Stop Fullscreen Aiming`
  (bind _camerawidgetref (`self.CameraWidgetRef`))
  ;[1 1 1] Fullscreen aiming logic ( called from CharacterBP)
  ;;[0 0.3259 0.5] Stop fullscreen aiming - reverse everything back to normal.
  (`Widget.SetVisibility` (`/Game/Market/AdvancedLightActors/Widgets/W_CameraScreen.BackgroundBorder` _camerawidgetref) "Visible")
  (`Widget.RemoveFromParent` _camerawidgetref)
  (`SceneComponent.K2_SetRelativeLocation` (`self.Camera`) (`self.DefaultCameraLocation`) false false)
  (`PlayerController.SetViewTargetWithBlend` (`GameplayStatics.GetPlayerController` 0) (`self.GetOwner`) 0.0 "VTBlend_Linear" 0.0 false)
  (`self.StopNightVision`)
  (`UserWidget.AddToViewport` (`self.HUDReference`) 0)
  (set `self.IsFullscreenAiming?` false))

(event `PhotogenicTargetLost`
  (bind _i_camera_focus (`/Game/Market/AdvancedLightActors/Widgets/W_CameraScreen.I_Camera_Focus` (`self.CameraWidgetRef`)))
  ;[1 1 1] Photo Creation Events
  ;;[0 0.3259 0.5] If the target is lost, reset everything to 0.
  (set `self.PhotoTargetActor` null)
  (set `self.PhotoTargetFound?` false)
  (set `self.SearchingForComponent?` false)
  (set `self.CanTakePhoto?` false)
  (`Image.SetBrushFromTexture` _i_camera_focus "/Game/Market/AdvancedLightActors/Widgets/Textures/T_Camera_Focus_Wide.T_Camera_Focus_Wide" true)
  (`Image.SetColorAndOpacity` _i_camera_focus (struct :`R` 1.0 :`G` 1.0 :`B` 1.0 :`A` 1.0)))

(event `IncrementDrainRate`
  (params (Amount :type "Float (double-precision)"))
  ;[1 1 1] Battery Related Events
  ;;[0 0.3259 0.5] Increment Drain Rate - make the battery drain down slower. because it waits more time on every tick.
  (set `self.CurrentDrainRate` (`KismetMathLibrary.FClamp` (+ (`self.CurrentDrainRate`) Amount) 0.0 (`self.Level1DrainRate`))))

(event `Update Recording Text`
  (params (`New Text` :type Text) (`Text Color` :type "LinearColor Structure"))
  (bind _t_recordingtext (`/Game/Market/AdvancedLightActors/Widgets/W_CameraScreen.T_RecordingText` (`self.CameraWidgetRef`)))
  ;[1 1 1] Recording Events
  ;;[0 0.3259 0.5] Update Recording Text - set the text to "STOP" or "REC" then set the color to green or red depending on the camera is currently recording or not.
  (`TextBlock.SetText` _t_recordingtext `New Text`)
  (`TextBlock.SetColorAndOpacity` _t_recordingtext (make `SlateColor` `Text Color`)))

(event `StopNightVision`
  (bind _scenecapturecomponent2d (`self.SceneCaptureComponent2D`))
  ;[1 1 1] Toggle NightVision On / Off
  ;;[0 0.3259 0.5] Stop Night Vision - Reverse everything back to default.
  (`self.IncrementDrainRate` (`self.NightVisionDrainRate`))
  (if (`self.IsFullscreenAiming?`)
    (set `PostProcessComponent.bEnabled` false (`self.NightVision`))
    (set `self.IsNightVisionOn?` false)
    (`Widget.SetVisibility` (`/Game/Market/AdvancedLightActors/Widgets/W_CameraScreen.I_NightVisionOn` (`self.CameraWidgetRef`)) "Hidden")
    (else
      (set `SceneCaptureComponent2D.PostProcessSettings` (`self.DefaultPPSettings`) _scenecapturecomponent2d)
      (set `SceneCaptureComponent2D.CaptureSource` "SCS_SceneColorSceneDepth" _scenecapturecomponent2d)
      (set `self.IsNightVisionOn?` false)
      (`Widget.SetVisibility` (`/Game/Market/AdvancedLightActors/Widgets/W_CameraScreen.I_NightVisionOn` (`self.CameraWidgetRef`)) "Hidden"))))

(event `TakePhoto`
  ;[1 1 1] Photo Creation Events
  ;;[0 0.3259 0.5] Take Photo ( T , RT) press. send the camera interaction started message to the target actor.
  (message `/Game/Market/AdvancedLightActors/Blueprints/Interfaces/BPI_CameraInteraction.CameraInteractionStarted` (`self.PhotoTargetActor`))
  (`/Game/Market/AdvancedLightActors/Widgets/W_CameraScreen.TakePhoto` (`self.CameraWidgetRef`))
  (`self.Server Play LightActor Sound` (`self.CameraPhotoSound`)))

(event `CameraZoomOut`
  (params (ZoomAmount :type "Float (double-precision)"))
  (bind _pb_zoomlevel (`/Game/Market/AdvancedLightActors/Widgets/W_CameraScreen.PB_ZoomLevel` (`self.CameraWidgetRef`)))
  (bind _fovangle (`SceneCaptureComponent2D.FOVAngle` (`self.SceneCaptureComponent2D`)))
  (bind _pb_zoomlevel_2 (`/Game/Market/AdvancedLightActors/Widgets/W_CameraScreen.PB_ZoomLevel` (`self.CameraWidgetRef`)))
  (bind _fieldofview (`CameraComponent.FieldOfView` (`self.Camera`)))
  ;[1 1 1] Camera Zoom In / Out Functions - From CharacterBP
  ;;[0 0.3259 0.5] Same as above, if the FOV is less than the max fov (90) - Zoom out by the zoom amount.
  (if (`self.IsFullscreenAiming?`)
    (if (< _fieldofview (`self.MaxZoomFOV`))
      (`CameraComponent.SetFieldOfView` (`self.Camera`) (+ _fieldofview ZoomAmount))
      (`ProgressBar.SetPercent` _pb_zoomlevel (- (`ProgressBar.Percent` _pb_zoomlevel) 0.25)))
    (elif (< _fovangle (`self.MaxZoomFOV`))
      (set `SceneCaptureComponent2D.FOVAngle` (+ _fovangle ZoomAmount) (`self.SceneCaptureComponent2D`))
      (`ProgressBar.SetPercent` _pb_zoomlevel_2 (- (`ProgressBar.Percent` _pb_zoomlevel_2) 0.25)))))

(event `self.Server Toggle Active Light`
  (bind _flashlightdrainrate (`self.FlashlightDrainRate`))
  (bind _i_flashlighton (`/Game/Market/AdvancedLightActors/Widgets/W_CameraScreen.I_FlashlightOn` (`self.CameraWidgetRef`)))
  ;[1 1 1] Overwritten Events from parent
  ;;[0 0.3259 0.5] Event Toggle Active Light - call the parent's function (turn on the flashlight), then set the FlashlightOn icon to visible, and make the battery drain out faster.
  (`parent.Server Toggle Active Light`)
  (if (`self.IsTurnedOn?`)
    (`Widget.SetVisibility` _i_flashlighton "Visible")
    (`self.DecrementDrainRate` _flashlightdrainrate)
    (else
      (`Widget.SetVisibility` _i_flashlighton "Hidden")
      (`self.IncrementDrainRate` _flashlightdrainrate))))

(event `/Game/Market/AdvancedLightActors/Blueprints/Interfaces/BPI_LightActors.Equipped`
  ;[1 1 1] Overwritten Events from parent
  ;;[0 0.3259 0.5] Update Battery Amount On Every Equip
  (`parent.Equipped`)
  (bind _battery_amount (message `/Game/Market/AdvancedLightActors/Blueprints/Interfaces/BPI_LightActors.GetBatteries` (`self.GetOwner`)))
  (`self.BatteryAmountChanged` _battery_amount))

(event `self.Multicast Restore Power`
  ;[1 1 1] Overwritten Events from parent
  ;;[0 0.3259 0.5] If a player puts in a new battery while equipped, it needs to update the battery counter.
  (`parent.Multicast Restore Power`)
  (bind _battery_amount (message `/Game/Market/AdvancedLightActors/Blueprints/Interfaces/BPI_LightActors.GetBatteries` (`self.GetOwner`)))
  (`self.BatteryAmountChanged` _battery_amount)
  (`/Game/Market/AdvancedLightActors/Widgets/W_CameraScreen.ToggleBatteryOutScreen` (`self.CameraWidgetRef`) false))

(event `self.MulticastLightActorOut`
  ;[1 1 1] Overwritten Events from parent
  ;;[0 0.3259 0.5] The Multicast LightActorOut code is overwritten from the LightActorMaster, to use the parent's event, then reset the camera, and show the battery out screen when the battery is out.
  (`parent.MulticastLightActorOut`)
  (`self.ResetCamera`)
  (`/Game/Market/AdvancedLightActors/Widgets/W_CameraScreen.ToggleBatteryOutScreen` (`self.CameraWidgetRef`) true))

(fn `CameraPhotoLineTrace`
  (bind _arrow (`self.Arrow`))
  (bind _returnvalue (`SceneComponent.K2_GetComponentLocation` _arrow))
  (bind _i_camera_focus (`/Game/Market/AdvancedLightActors/Widgets/W_CameraScreen.I_Camera_Focus` (`self.CameraWidgetRef`)))
  ;[1 1 1] Similar to the InteractionLineTrace, this line trace searches for the specific component in an actor.
  ;;[0 0.3259 0.5] Same as before, line trace from camera's location forward.
  (bind _debuggingon_ (message `/Game/Market/AdvancedLightActors/Blueprints/Interfaces/BPI_DeveloperOptions.GetIsDebuggingOn?` (`self.GetOwner`)))
  (bind (_outhit _returnvalue_2) (`KismetSystemLibrary.LineTraceSingle` :`Start` _returnvalue :`End` (+ _returnvalue (* (`SceneComponent.GetForwardVector` _arrow) (`self.InteractionDistance`))) :`TraceChannel` "TraceTypeQuery1" :`DrawDebugType` (select `bool` _debuggingon_ :`true` "ForDuration" :!type "EDrawDebugTrace Enum")))
  ;;[0 0.3259 0.5] If the found actor has the BPI_CameraInteractions in it, check if it's required component is the same as the one the trace hits.
  (if _returnvalue_2
    (bind (_bblockinghit _binitialoverlap _time _distance _location _impactpoint _normal _impactnormal _physmat _hitactor _hitcomponent) (`GameplayStatics.BreakHitResult` _outhit))
    (if (`KismetSystemLibrary.DoesImplementInterface` _hitactor "/Game/Market/AdvancedLightActors/Blueprints/Interfaces/BPI_CameraInteraction.BPI_CameraInteraction_C")
      (bind (_needsspecificcomponent_ _requiredcomponent) (message `/Game/Market/AdvancedLightActors/Blueprints/Interfaces/BPI_CameraInteraction.GetPhotoActorDetails` _hitactor))
      (if (== _requiredcomponent _hitcomponent)
        ;;[0 0.3259 0.5] If the trace found the right component, enable the photo creation process.
        (if (not (`self.CanTakePhoto?`))
          (`KismetSystemLibrary.PrintString` "Component Found!")
          (`Image.SetColorAndOpacity` _i_camera_focus (struct :`R` 0.002465 :`G` 1.0 :`A` 1.0))
          (set `self.CanTakePhoto?` true))
        (else
          ;;[0 0.3259 0.5] If the trace is hitting the good actor, but the wrong component,  call this code.
          (`KismetSystemLibrary.PrintString` "Wrong Component! Search for an other one.")
          (set `self.CanTakePhoto?` false)
          (`Image.SetColorAndOpacity` _i_camera_focus (struct :`R` 0.5 :`B` 0.002984 :`A` 1.0))))
      (else
        ;;;[0 0.3259 0.5] If the line trace hits an other actor without the tag, but has hit the required actor at least once, call the target lost code again.
        (`/Engine/EditorBlueprintResources/StandardMacros.IsValid` (`self.PhotoTargetActor`)
          (:`Is Valid`
            (`self.PhotogenicTargetLost`)))))
    (else
      ;;[0 0.3259 0.5] the line trace doesn't hit the actor anymore, (but hit it before at least once) it calls the target lost code.
      (`/Engine/EditorBlueprintResources/StandardMacros.IsValid` (`self.PhotoTargetActor`)
        (:`Is Valid`
          (`self.PhotogenicTargetLost`))))))

(fn `InteractionLineTrace`
  (locals (LocalHitActor :type "Actor Object Reference"))
  (bind _arrow (`self.Arrow`))
  (bind _localhitactor (`local.LocalHitActor`))
  (bind _returnvalue (`SceneComponent.K2_GetComponentLocation` _arrow))
  ;[1 1 1] Called from Event Tick - searches for interactable targets (Actors with Interface BPI_CameraInteractions)
  ;;[0 0.3259 0.5] Line trace from the camera arrow's location
  (bind _debuggingon_ (message `/Game/Market/AdvancedLightActors/Blueprints/Interfaces/BPI_DeveloperOptions.GetIsDebuggingOn?` (`self.GetOwner`)))
  (bind (_outhit _returnvalue_2) (`KismetSystemLibrary.LineTraceSingle` :`Start` _returnvalue :`End` (+ _returnvalue (* (`SceneComponent.GetForwardVector` _arrow) (`self.InteractionDistance`))) :`TraceChannel` "TraceTypeQuery1" :`DrawDebugType` (select `bool` _debuggingon_ :`true` "ForDuration" :!type "EDrawDebugTrace Enum")))
  ;;[0 0.3259 0.5] Only accept actors with Interface BPI_CameraInteractions. if the actor has "Photo" tag, get it's details, meaning the actor should be photographed, not just recorded.if not photoable, the system can start the interaction
  (if _returnvalue_2
    (bind (_bblockinghit _binitialoverlap _time _distance _location _impactpoint _normal _impactnormal _physmat _hitactor) (`GameplayStatics.BreakHitResult` _outhit))
    (set `local.LocalHitActor` _hitactor)
    (if (`KismetSystemLibrary.DoesImplementInterface` _hitactor "/Game/Market/AdvancedLightActors/Blueprints/Interfaces/BPI_CameraInteraction.BPI_CameraInteraction_C")
      (if (`self.ActorHasTag` _hitactor "Photo")
        ;;[0 0.3259 0.5] If the target has the photo tag, get it's details and run the photo taking logic. If it doesn't have the tag, start the interaction immediately.
        (bind _needsspecificcomponent_ (message `/Game/Market/AdvancedLightActors/Blueprints/Interfaces/BPI_CameraInteraction.GetPhotoActorDetails` _localhitactor))
        (`self.PhotogenicTargetFound` _localhitactor _needsspecificcomponent_)
        (else
          (message `/Game/Market/AdvancedLightActors/Blueprints/Interfaces/BPI_CameraInteraction.CameraInteractionStarted` (`local.LocalHitActor`))))
      (else
        (`/Engine/EditorBlueprintResources/StandardMacros.IsValid` (`self.PhotoTargetActor`) :!label _label
          (:`Is Valid`
            (`self.PhotogenicTargetLost`)))))
    (else
      (goto _label))))

(fn `ResetCamera`
  ;[1 1 1] Reset Camera Function - called when battery drains down to 0. If any function is on at the moment, turn it off. Then, send message to the owner(player) that the camera is out. (Event written in CharacterBP)
  (if (`self.IsTurnedOn?`)
    (`self.Server Toggle Active Light`))
  (if (`self.IsNightVisionOn?`)
    (`self.StopNightVision`))
  (if (`self.IsRecording?`)
    (`self.StopRecording`))
  (message `/Game/Market/AdvancedLightActors/Blueprints/Interfaces/BPI_LightActors.CameraOut` (`self.GetOwner`)))

(fn `UserConstructionScript`
  (`parent.UserConstructionScript`))