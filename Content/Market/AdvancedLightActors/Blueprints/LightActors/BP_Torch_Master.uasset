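; BP_Torch_Master is the base torch light actor, extending a parent light Blueprint with a fire particle effect that follows the torch's lit state.
; On BeginPlay it runs the parent logic, then sets its point light as the active light component.
; The overridden Turnedon and TurnedOff interface events call a server event, which multicasts activation or deactivation of the fire particle system so the effect is replicated.
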(event `Server Toggle Active Particle System`
  (params (`On?` :type Boolean))
  ;[0 0.3259 0.5] Replicated Particle System Toggling
  (`self.Multicast Toggle Active Particle System` `On?`))

(event `self.ReceiveBeginPlay`
  ;[0 0.3259 0.5] On beginplay - set the active light component to the point light.
  (`parent.ReceiveBeginPlay`)
  (set `self.ActiveLightComponent` (`self.PointLight`)))

(event `/Game/Market/AdvancedLightActors/Blueprints/Interfaces/BPI_LightActors.TurnedOn`
  ;[0 0.3259 0.5] Interface Overwritten events - replicated toggling the fire particle when igniting/putting out the torch.
  (`self.Server Toggle Active Particle System` true))

(event `Multicast Toggle Active Particle System`
  (params (`On?` :type Boolean))
  (bind _ps_torch_fire (`self.PS_Torch_Fire`))
  ;[0 0.3259 0.5] Replicated Particle System Toggling
  (if `On?`
    (`ActorComponent.Activate` _ps_torch_fire false)
    (else
      (`ActorComponent.Deactivate` _ps_torch_fire))))

(event `/Game/Market/AdvancedLightActors/Blueprints/Interfaces/BPI_LightActors.TurnedOff`
  ;[0 0.3259 0.5] Interface Overwritten events - replicated toggling the fire particle when igniting/putting out the torch.
  (`self.Server Toggle Active Particle System` false))

(fn `UserConstructionScript`
  (`parent.UserConstructionScript`))