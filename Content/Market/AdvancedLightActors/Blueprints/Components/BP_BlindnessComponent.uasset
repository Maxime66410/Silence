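; Actor component that blinds a locally controlled player by fading a full-screen W_BlindedImage overlay with the accumulated blindness amount.
; AddBlindnessAmount adds to a clamped value while CanBeBlinded is true, then creates or updates the widget.
; A retriggerable delay postpones recovery until hits stop, then a timed loop decrements the value, blocking new blindness until it reaches zero and the widget is removed.
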(event `Add Blindness Amount`
  (params (`Amount To Add` :type "Float (double-precision)") (Pawn :type "Pawn Object Reference"))
  ;[1 1 1] Add Blindness Amount
  ;;[0 0.3259 0.5] First Check if the player is locally controlled. (Make sure we won't create the widget that draws the image to the screen later to the player character who blinded the other one.)
  (if (`Pawn.IsLocallyControlled` Pawn)
    ;;[0 0.3259 0.5] Then  add the amount to the blinded amount variable if the player can be blinded. (He can't be if he is already blinded or is recovering from blindness.)
    (if (`self.CanBeBlinded?`)
      (set `self.BlindedAmount` (`KismetMathLibrary.FClamp` (+ (`self.BlindedAmount`) `Amount To Add`) 0.0 100.0))
      ;;[0 0.3259 0.5] Then start creating or update the blindness widget.
      (`self.Update Blindness Widget`))))

(event `Update Blindness Widget`
  ;[1 1 1] Update Blindness Widget
  ;;[0 0.3259 0.5] Check if the widget is already drawn to the screen
  (`/Engine/EditorBlueprintResources/StandardMacros.IsValid` (`self.BlindedImageRef`)
    (:`Is Valid`
      _)
    (:`Is Not Valid`
      ;;[0 0.3259 0.5] If it isn't, then create it (this means this is the first time the actor is getting blinded) and create a reference.
      (bind _returnvalue (`|CreateWidget` "/Game/Market/AdvancedLightActors/Widgets/W_BlindedImage.W_BlindedImage_C" (`GameplayStatics.GetPlayerController` 0)))
      (bind _output_get (set `self.BlindedImageRef` _returnvalue))
      (`UserWidget.AddToViewport` _output_get 0)))
  ;;[0 0.3259 0.5] Then update the opacity of the image in the widget
  (`/Game/Market/AdvancedLightActors/Widgets/W_BlindedImage.Update Blinded Opacity` (`self.BlindedImageRef`) (`self.BlindedAmount`))
  ;;[0 0.3259 0.5] After 1 sec, if the player doesn't get blinded again, start recovering from it.
  (`KismetSystemLibrary.RetriggerableDelay` 1.0)
  (`self.Decrement Blinded Value` (`self.BlindnessDecrementValue`))
  (set `self.CanBeBlinded?` false))

(event `Decrement Blinded Value`
  (params (Amount :type "Float (double-precision)"))
  (bind _blindedamount (`self.BlindedAmount`))
  ;[1 1 1] Recursively Decrement Blindness Value
  ;;[0 0.3259 0.5] Decrement the blindness value with the amount
  (set `self.BlindedAmount` (`KismetMathLibrary.FClamp` (- (`self.BlindedAmount`) Amount) 0.0 100.0) :!label _label)
  ;;[0 0.3259 0.5] If the blindness widget is added to the screen (should be), update it's opacity
  (`/Engine/EditorBlueprintResources/StandardMacros.IsValid` (`self.BlindedImageRef`)
    (:`Is Valid`
      (`/Game/Market/AdvancedLightActors/Widgets/W_BlindedImage.Update Blinded Opacity` (`self.BlindedImageRef`) _blindedamount)
      ;;[0 0.3259 0.5] Check if the value got decremented until 0
      (if (<= _blindedamount 0.0)
        ;;[0 0.3259 0.5] If it is, exit the recursive function, and remove the widget, and make the player blindable again.
        (`Widget.RemoveFromParent` (`self.BlindedImageRef`))
        (set `self.BlindedImageRef` null)
        (set `self.CanBeBlinded?` true)
        (else
          ;;[0 0.3259 0.5] If it isn't 0 yet, wait 0.2 seconds, and decrement the value again until it reaches 0
          (`KismetSystemLibrary.RetriggerableDelay` 0.2)
          (goto _label))))))