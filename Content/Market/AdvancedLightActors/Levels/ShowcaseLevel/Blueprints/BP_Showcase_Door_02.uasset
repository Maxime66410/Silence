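; BP_Showcase_Door_02 is a double sliding door for the Advanced Light Actors showcase level that opens automatically when the player is near.
; BeginPlay caches both panels' relative start locations, and a timeline lerps them in opposite directions by DestinationLocation.
; OverlapTrigger plays the timeline from the start when the player character enters and reverses it on exit.
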(event `self.ReceiveBeginPlay`
  (set `self.LeftDoorStartLocation` (`SceneComponent.RelativeLocation` (`self.LeftDoor`)))
  (set `self.RightDoorStartLocation` (`SceneComponent.RelativeLocation` (`self.RightDoor`))))

(event `PlayDoorOpening`
  (bind (_direction _alpha) (`Timeline|DoorOpeningTimeline` :!via `PlayFromStart` :!label _label)
    (:`Update`
      (`SceneComponent.K2_SetRelativeLocation` (`self.RightDoor`) (`KismetMathLibrary.VLerp` (`self.RightDoorStartLocation`) (+ (`self.RightDoorStartLocation`) (`self.DestinationLocation`)) _alpha) false false)
      (`SceneComponent.K2_SetRelativeLocation` (`self.LeftDoor`) (`KismetMathLibrary.VLerp` (`self.LeftDoorStartLocation`) (- (`self.LeftDoorStartLocation`) (`self.DestinationLocation`)) _alpha) false false))))

(event `CloseDoor`
  (goto _label :!via `Reverse`))

(event `self.OverlapTrigger.OnComponentBeginOverlap`
  (params (OverlappedComponent :type "PrimitiveComponent Object Reference") (OtherActor :type "Actor Object Reference") (OtherComp :type "PrimitiveComponent Object Reference") (OtherBodyIndex :type Integer) (bFromSweep :type Boolean) (SweepResult :type "HitResult Structure (by ref)"))
  (if (== OtherActor (`GameplayStatics.GetPlayerCharacter` 0))
    (`self.PlayDoorOpening`)))

(event `self.OverlapTrigger.OnComponentEndOverlap`
  (params (OverlappedComponent :type "PrimitiveComponent Object Reference") (OtherActor :type "Actor Object Reference") (OtherComp :type "PrimitiveComponent Object Reference") (OtherBodyIndex :type Integer))
  (if (== OtherActor (`GameplayStatics.GetPlayerCharacter` 0))
    (`self.CloseDoor`)))

(fn `UserConstructionScript`)