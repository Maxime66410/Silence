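; BP_ReigniteTorch is a showcase-level interactable that lets the player relight a held torch that has gone out.
; Its overlap trigger stores player character 0 and enables input on entry, then disables input on exit.
; Pressing Interact calls MulticastIgniteTorch, which casts to the example flashlight character and, if its light actor is an unlit Torch, restores power, toggles it and calls its turned-on message.
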(event `Multicast IgniteTorch`
  (bind _asbp_example_flashlight_character (cast `/Game/Market/AdvancedLightActors/Blueprints/CharacterBP/BP_ExampleFlashlightCharacter` (`self.OverlappedPlayer`)))
  (bind _lightactorref (`/Game/Market/AdvancedLightActors/Blueprints/CharacterBP/BP_ExampleFlashlightCharacter.LightActorRef` _asbp_example_flashlight_character))
  (`/Engine/EditorBlueprintResources/StandardMacros.IsValid` _lightactorref
    (:`Is Valid`
      (if (not (`/Game/Market/AdvancedLightActors/Blueprints/LightActors/BP_LightActor_Master.IsTurnedOn?` _lightactorref))
        (switch `/Game/Market/AdvancedLightActors/Blueprints/E_LightActorTypes` (`/Game/Market/AdvancedLightActors/Blueprints/LightActors/BP_LightActor_Master.LightActorType` _lightactorref)
          (:`NewEnumerator3`
            (`/Game/Market/AdvancedLightActors/Blueprints/LightActors/BP_LightActor_Master.Server Restore Power` _lightactorref)
            (`/Game/Market/AdvancedLightActors/Blueprints/LightActors/BP_LightActor_Master.Server Toggle Active Light` _lightactorref)
            (message `/Game/Market/AdvancedLightActors/Blueprints/Interfaces/BPI_LightActors.TurnedOn` _lightactorref)))))))

(event `self.OverlapTrigger.OnComponentBeginOverlap`
  (params (OverlappedComponent :type "PrimitiveComponent Object Reference") (OtherActor :type "Actor Object Reference") (OtherComp :type "PrimitiveComponent Object Reference") (OtherBodyIndex :type Integer) (bFromSweep :type Boolean) (SweepResult :type "HitResult Structure (by ref)"))
  (if (== OtherActor (`GameplayStatics.GetPlayerCharacter` 0))
    (set `self.OverlappedPlayer` OtherActor)
    (`self.EnableInput` (`GameplayStatics.GetPlayerController` 0))))

(event `self.OverlapTrigger.OnComponentEndOverlap`
  (params (OverlappedComponent :type "PrimitiveComponent Object Reference") (OtherActor :type "Actor Object Reference") (OtherComp :type "PrimitiveComponent Object Reference") (OtherBodyIndex :type Integer))
  (if (== (`GameplayStatics.GetPlayerCharacter` 0) OtherActor)
    (set `self.OverlappedPlayer` OtherActor)
    (`self.DisableInput` (`GameplayStatics.GetPlayerController` 0))))

(event `InputAction|Interact`
  (params (Key :type "Key Structure"))
  (:`Pressed`
    (`self.Multicast IgniteTorch`)))

(fn `UserConstructionScript`)