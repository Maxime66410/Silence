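; Showcase-level teleporter actor that moves the player to a destination component when they step into its trigger volume.
; CollisionTrigger's begin overlap checks that the other actor is the first player character and casts it to BP_ExampleFlashlightCharacter.
; It stores that character as the target, then TeleportPlayerToLocation teleports it to PlayerDestination's world location and rotation.
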(event `TeleportPlayerToLocation`
  (bind _playerdestination (`self.PlayerDestination`))
  (`self.K2_TeleportTo` (`self.TargetToTeleport`) (`SceneComponent.K2_GetComponentLocation` _playerdestination) (`SceneComponent.K2_GetComponentRotation` _playerdestination)))

(event `self.CollisionTrigger.OnComponentBeginOverlap`
  (params (OverlappedComponent :type "PrimitiveComponent Object Reference") (OtherActor :type "Actor Object Reference") (OtherComp :type "PrimitiveComponent Object Reference") (OtherBodyIndex :type Integer) (bFromSweep :type Boolean) (SweepResult :type "HitResult Structure (by ref)"))
  (if (== OtherActor (`GameplayStatics.GetPlayerCharacter` 0))
    (bind _asbp_example_flashlight_character (cast `/Game/Market/AdvancedLightActors/Blueprints/CharacterBP/BP_ExampleFlashlightCharacter` OtherActor))
    (set `self.TargetToTeleport` _asbp_example_flashlight_character)
    (`self.TeleportPlayerToLocation`)))

(fn `UserConstructionScript`)