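; BP_PhotoAbleCube_02 is a showcase-level actor that responds to camera interaction by triggering other actors.
; The first CameraInteractionStarted event passes a DoOnce and sends StartInteractionMessage to every entry in the TargetActor array.
; GetPhotoActorDetails reports whether a specific component is needed and names Lantern as the required one.
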(event `/Game/Market/AdvancedLightActors/Blueprints/Interfaces/BPI_CameraInteraction.CameraInteractionStarted`
  (bind _targetactor (`self.TargetActor`))
  (`/Engine/EditorBlueprintResources/StandardMacros.DoOnce` false
    (:`Completed`
      (if (> (`KismetArrayLibrary.Array_Length` _targetactor) 0)
        (for _array_element _targetactor
          (message `/Game/Market/AdvancedLightActors/Blueprints/Interfaces/BPI_CameraInteraction.StartInteraction` _array_element))))))

(fn `GetPhotoActorDetails`
  (returns (`NeedsSpecificComponent?` :type Boolean) (RequiredComponent :type "ActorComponent Object Reference"))
  (return (`self.NeedsSpecificComponent?`) (`self.Lantern`)))

(fn `UserConstructionScript`)