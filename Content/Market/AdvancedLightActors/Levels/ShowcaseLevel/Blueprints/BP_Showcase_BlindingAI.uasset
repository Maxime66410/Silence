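; Showcase light that the player can switch on and off to demonstrate blinding of actors such as AI.
; An overlap trigger stores the player, enables Interact input and shows prompt text; Interact toggles both lights through a multicast-named event.
; While lit, Tick runs a delayed forward sphere trace, using BPI_FlashlightBlinding to match the hit against the target's head bone and increment its blindness.
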(event `InputAction|Interact`
  (params (Key :type "Key Structure"))
  (:`Pressed`
    (`self.Multicast Toggle Turned On`)))

(event `self.ReceiveTick`
  (params (DeltaSeconds :type "Float (single-precision)"))
  (if (`self.IsTurnedOn?`)
    (`KismetSystemLibrary.Delay` 0.1)
    (`self.BlindnessSphereTrace`)))

(event `Multicast Toggle Turned On`
  (bind _sourcelight (`self.SourceLight`))
  (bind _spotlight (`self.SpotLight`))
  (if (`self.IsTurnedOn?`)
    (set `self.IsTurnedOn?` false)
    (`LightComponent.SetIntensity` _sourcelight 0.0)
    (`LightComponent.SetIntensity` _spotlight 0.0)
    (else
      (set `self.IsTurnedOn?` true)
      (`LightComponent.SetIntensity` _sourcelight 5000.0)
      (`LightComponent.SetIntensity` _spotlight 10000.0))))

(event `self.OverlapTrigger.OnComponentBeginOverlap`
  (params (OverlappedComponent :type "PrimitiveComponent Object Reference") (OtherActor :type "Actor Object Reference") (OtherComp :type "PrimitiveComponent Object Reference") (OtherBodyIndex :type Integer) (bFromSweep :type Boolean) (SweepResult :type "HitResult Structure (by ref)"))
  (if (== OtherActor (`GameplayStatics.GetPlayerCharacter` 0))
    (bind _asbp_example_flashlight_character (cast `/Game/Market/AdvancedLightActors/Blueprints/CharacterBP/BP_ExampleFlashlightCharacter` OtherActor))
    (set `self.PlayerRef` _asbp_example_flashlight_character)
    (`self.EnableInput` (`GameplayStatics.GetPlayerController` 0))
    (`SceneComponent.SetHiddenInGame` (`self.TextRender`) false false)))

(event `self.OverlapTrigger.OnComponentEndOverlap`
  (params (OverlappedComponent :type "PrimitiveComponent Object Reference") (OtherActor :type "Actor Object Reference") (OtherComp :type "PrimitiveComponent Object Reference") (OtherBodyIndex :type Integer))
  (if (== (stale `self.OverlapTrigger.OnComponentBeginOverlap` OtherActor) (`GameplayStatics.GetPlayerCharacter` 0))
    (`self.DisableInput` (`GameplayStatics.GetPlayerController` 0))
    (`SceneComponent.SetHiddenInGame` (`self.TextRender`) true false)))

(fn `BlindnessSphereTrace`
  (bind _arrow (`self.Arrow`))
  (bind _playerref (`self.PlayerRef`))
  (bind _returnvalue (`SceneComponent.K2_GetComponentLocation` _arrow))
  ;[1 1 1] Blinding Sphere Trace- used in Flashlight T1 and T2 when aiming with flashlight
  ;;[0 0.3259 0.5] Same Locations as light flickering
  (`/Engine/EditorBlueprintResources/StandardMacros.IsValid` _playerref
    (:`Is Valid`
      (bind (_outhit _returnvalue_2) (`KismetSystemLibrary.SphereTraceSingle` :`Start` _returnvalue :`End` (+ _returnvalue (* (`SceneComponent.GetForwardVector` _arrow) 1200.0)) :`Radius` 15.0 :`TraceChannel` "TraceTypeQuery1" :`DrawDebugType` (select `bool` (`/Game/Market/AdvancedLightActors/Blueprints/CharacterBP/BP_ExampleFlashlightCharacter.DebuggingOn?` _playerref) :`true` "ForDuration" :!type "EDrawDebugTrace Enum") :`TraceColor` (struct :`R` 0.5 :`B` 0.002984 :`A` 1.0)))
      ;;[0 0.3259 0.5] Check if the actor has the BPI_FlashlightBlindness interface in it, and check if the trace hits the head bone of the actor. (send a message to the actor the trace hits.) this message needs to be written in each actor. it needs to return the head bone of the mesh. (check it in the skeleton, then write it in.)
      (if _returnvalue_2
        (bind (_bblockinghit _binitialoverlap _time _distance _location _impactpoint _normal _impactnormal _physmat _hitactor _hitcomponent _hitbonename) (`GameplayStatics.BreakHitResult` _outhit))
        (if (`KismetSystemLibrary.DoesImplementInterface` _hitactor "/Game/Market/AdvancedLightActors/Blueprints/Interfaces/BPI_FlashlightBlinding.BPI_FlashlightBlinding_C")
          (bind _headbonename (message `/Game/Market/AdvancedLightActors/Blueprints/Interfaces/BPI_FlashlightBlinding.GetHeadBone` _hitactor))
          (if (== _headbonename _hitbonename)
            ;;[0 0.3259 0.5] Then increment the blindness value of the actor. (event needs to be written in the actor)
            (message `/Game/Market/AdvancedLightActors/Blueprints/Interfaces/BPI_FlashlightBlinding.IncrementBlindedValue` _hitactor 10.0)))))))

(fn `UserConstructionScript`)