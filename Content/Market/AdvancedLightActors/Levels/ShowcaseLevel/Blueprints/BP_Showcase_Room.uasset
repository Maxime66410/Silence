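; Modular room actor for the AdvancedLightActors showcase level, assembled from instance flags in the construction script.
; Each enabled wall adds a mesh at its spawn point, stored in SpawnedWallArray, with a child actor added for door variants.
; Front, right and left doors get styled room-title text, while back-wall text has its own toggle.
; Optional ceiling and separated-room meshes complete the room; the event graph has no runtime logic.
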(event `self.ReceiveTick`
  (params (DeltaSeconds :type "Float (single-precision)"))
  (if true
    _))

(fn `UserConstructionScript`
  (bind _spawnedwallarray (`self.SpawnedWallArray`))
  (bind _spawnedwallarray_2 (`self.SpawnedWallArray`))
  (bind _spawnedwallarray_3 (`self.SpawnedWallArray`))
  (bind _spawnedwallarray_4 (`self.SpawnedWallArray`))
  (bind _returnvalue (`SceneComponent.GetRelativeTransform` (`self.LeftWallSpawnPoint`)))
  (bind _returnvalue_2 (`SceneComponent.GetRelativeTransform` (`self.RightWallSpawnPoint`)))
  (bind _returnvalue_3 (`SceneComponent.GetRelativeTransform` (`self.FrontWallSpawnPoint`)))
  (bind _returnvalue_4 (`SceneComponent.GetRelativeTransform` (`self.BackWallSpawnPoint`)))
  (if (`self.SeperatedRoom?`)
    (`AddComponent|NODE_AddStaticMeshComponent-14` :`RelativeTransform` (`KismetMathLibrary.MakeTransform` (0.0 0.0 0.0))))
  (if (`self.FrontWall?`)
    (if (`self.ReplaceFWallsToDoors`)
      (bind _returnvalue_5 (`AddComponent|NODE_AddStaticMeshComponent-7` :`RelativeTransform` _returnvalue_3))
      (`KismetArrayLibrary.Array_Add` _spawnedwallarray _returnvalue_5)
      (`AddComponent|NODE_AddChildActorComponent-1` :`RelativeTransform` _returnvalue_3)
      (bind _returnvalue_6 (`AddComponent|NODE_AddTextRenderComponent-1` :`RelativeTransform` (`KismetMathLibrary.MakeTransform` (950.0 0.0 435.0) (struct :`Yaw` 180.0))))
      (`TextRenderComponent.K2_SetText` _returnvalue_6 (`self.FrontRoomTitleText`))
      (`TextRenderComponent.SetWorldSize` _returnvalue_6 (`self.NextRoomTitleSize`))
      (`TextRenderComponent.SetTextRenderColor` _returnvalue_6 (`self.NextRoomTitleColor`))
      (else
        (bind _returnvalue_7 (`AddComponent|NODE_AddStaticMeshComponent-0` :`RelativeTransform` _returnvalue_3))
        (`KismetArrayLibrary.Array_Add` _spawnedwallarray _returnvalue_7))))
  (if (`self.BackWall?`)
    (if (`self.ReplaceBWallsToDoors`)
      (bind _returnvalue_8 (`AddComponent|NODE_AddStaticMeshComponent-8` :`RelativeTransform` _returnvalue_4))
      (`KismetArrayLibrary.Array_Add` _spawnedwallarray_2 _returnvalue_8)
      (`AddComponent|NODE_AddChildActorComponent-4` :`RelativeTransform` _returnvalue_4)
      (else
        (bind _returnvalue_9 (`AddComponent|NODE_AddStaticMeshComponent-1` :`RelativeTransform` _returnvalue_4))
        (`KismetArrayLibrary.Array_Add` _spawnedwallarray_2 _returnvalue_9))))
  (if (`self.BackWallText?`)
    (bind _returnvalue_10 (`AddComponent|NODE_AddTextRenderComponent-5` :`RelativeTransform` (`KismetMathLibrary.MakeTransform` (-950.0 0.0 435.0))))
    (`TextRenderComponent.K2_SetText` _returnvalue_10 (`self.BackRoomTitleText`))
    (`TextRenderComponent.SetWorldSize` _returnvalue_10 (`self.BackRoomTitleSize`))
    (`TextRenderComponent.SetTextRenderColor` _returnvalue_10 (`self.BackRoomTitleColor`)))
  (if (`self.RightWall?`)
    (if (`self.ReplaceRWallsToDoors`)
      (bind _returnvalue_11 (`AddComponent|NODE_AddStaticMeshComponent-9` :`RelativeTransform` _returnvalue_2))
      (`KismetArrayLibrary.Array_Add` _spawnedwallarray_3 _returnvalue_11)
      (`AddComponent|NODE_AddChildActorComponent-2` :`RelativeTransform` _returnvalue_2)
      (bind _returnvalue_12 (`AddComponent|NODE_AddTextRenderComponent-2` :`RelativeTransform` (`KismetMathLibrary.MakeTransform` (0.0 950.0 435.0) (struct :`Yaw` 270.0))))
      (`TextRenderComponent.K2_SetText` _returnvalue_12 (`self.RightRoomTitleText`))
      (`TextRenderComponent.SetWorldSize` _returnvalue_12 (`self.NextRoomTitleSize`))
      (`TextRenderComponent.SetTextRenderColor` _returnvalue_12 (`self.NextRoomTitleColor`))
      (else
        (bind _returnvalue_13 (`AddComponent|NODE_AddStaticMeshComponent-2` :`RelativeTransform` _returnvalue_2))
        (`KismetArrayLibrary.Array_Add` _spawnedwallarray_3 _returnvalue_13))))
  (if (`self.LeftWall?`)
    (if (`self.ReplaceLWallsToDoors`)
      (bind _returnvalue_14 (`AddComponent|NODE_AddStaticMeshComponent-10` :`RelativeTransform` _returnvalue))
      (`KismetArrayLibrary.Array_Add` _spawnedwallarray_4 _returnvalue_14)
      (`AddComponent|NODE_AddChildActorComponent-3` :`RelativeTransform` _returnvalue)
      (bind _returnvalue_15 (`AddComponent|NODE_AddTextRenderComponent-3` :`RelativeTransform` (`KismetMathLibrary.MakeTransform` (0.0 -950.0 435.0) (struct :`Yaw` 90.0))))
      (`TextRenderComponent.K2_SetText` _returnvalue_15 (`self.LeftRoomTitleText`))
      (`TextRenderComponent.SetWorldSize` _returnvalue_15 (`self.NextRoomTitleSize`))
      (`TextRenderComponent.SetTextRenderColor` _returnvalue_15 (`self.NextRoomTitleColor`))
      (else
        (bind _returnvalue_16 (`AddComponent|NODE_AddStaticMeshComponent-3` :`RelativeTransform` _returnvalue))
        (`KismetArrayLibrary.Array_Add` _spawnedwallarray_4 _returnvalue_16))))
  (if (`self.SpawnCeiling?`)
    (`AddComponent|NODE_AddStaticMeshComponent-5` :`RelativeTransform` (`KismetMathLibrary.MakeTransform` (0.0 0.0 340.0)))))