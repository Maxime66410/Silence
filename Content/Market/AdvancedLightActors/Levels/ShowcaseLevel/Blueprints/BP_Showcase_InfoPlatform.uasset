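; BP_Showcase_InfoPlatform is an info display for the Advanced Light Actors showcase level, presenting title text, description text or an image.
; The construction script does all the work, hiding the title and description in game when their flags are off.
; ShowShowcaseImage swaps the description for an image plane and a Paper2D sprite set from SpriteToShow, and otherwise hides both image components.
; The event graph holds no logic.
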(fn `UserConstructionScript`
  (bind _imageplane (`self.ImagePlane`))
  (if (not (`self.HasTitleText?`))
    (`SceneComponent.SetHiddenInGame` (`self.TitleText`) true false))
  (if (not (`self.HasLongDescriptionText?`))
    (`SceneComponent.SetHiddenInGame` (`self.ShowcaseText`) true false))
  (if (`self.ShowShowcaseImage?`)
    (`SceneComponent.SetVisibility` _imageplane true false)
    (`SceneComponent.SetVisibility` (`self.PaperSprite`) true false)
    (`SceneComponent.SetVisibility` (`self.ShowcaseText`) false false)
    (`PaperSpriteComponent.SetSprite` (`self.PaperSprite`) (`self.SpriteToShow`))
    (else
      (`SceneComponent.SetVisibility` _imageplane false false)
      (`SceneComponent.SetVisibility` (`self.PaperSprite`) false false))))