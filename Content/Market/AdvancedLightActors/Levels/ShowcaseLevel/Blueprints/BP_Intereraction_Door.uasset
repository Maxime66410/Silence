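; Interactable sliding door actor for the AdvancedLightActors showcase level.
; It caches the door mesh's relative location at BeginPlay, and StartInteraction plays a timeline from the start that lerps the mesh toward that position plus DestinationLocation.
; The movement is one-way with no close logic, and GetPhotoActorDetails reports that no specific component is needed.
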(event `self.ReceiveBeginPlay`
  (set `self.RightDoorStartLocation` (`SceneComponent.RelativeLocation` (`self.DoorMesh`))))

(event `/Game/Market/AdvancedLightActors/Blueprints/Interfaces/BPI_CameraInteraction.StartInteraction`
  (bind (_direction _alpha) (`Timeline|Timeline_0` :!via `PlayFromStart`)
    (:`Update`
      (`SceneComponent.K2_SetRelativeLocation` (`self.DoorMesh`) (`KismetMathLibrary.VLerp` (`self.RightDoorStartLocation`) (+ (`self.RightDoorStartLocation`) (`self.DestinationLocation`)) _alpha) false false))))

(fn `GetPhotoActorDetails`
  (returns (`NeedsSpecificComponent?` :type Boolean) (RequiredComponent :type "ActorComponent Object Reference"))
  (return false null))

(fn `UserConstructionScript`)